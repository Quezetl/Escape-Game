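; Shop actor that shows a shop menu while the player's pawn is inside its Box trigger.
; On BeginPlay it waits briefly, then caches the player controller as a GameplayPC.
; Box overlap events check whether that controller's pawn is overlapping, adding the controller-owned ShopMenuWB widget to the viewport on entry and removing it on exit.
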(event OnComponentBeginOverlap(Box)
  (params (OverlappedComponent :type Primitive%20Component%20Object%20Reference) (OtherActor :type Actor%20Object%20Reference) (OtherComp :type Primitive%20Component%20Object%20Reference) (OtherBodyIndex :type Integer) (bFromSweep :type Boolean) (SweepResult :type Hit%20Result%20Structure%20%28by%20ref%29))
  (if (Collision|IsOverlappingActor OverlappedComponent (Pawn|GetControlledPawn (Variables|Default|GetPlayerControllerREF)) :!class /Script/Engine.PrimitiveComponent)
    (UserInterface|Viewport|AddtoViewport (Variables|/Game/Blueprints/Gameplay/GameplayPC.GameplayPC_C|GetShopMenuWB (Variables|Default|GetPlayerControllerREF)) 0)))

(event OnComponentEndOverlap(Box)
  (params (OverlappedComponent :type Primitive%20Component%20Object%20Reference) (OtherActor :type Actor%20Object%20Reference) (OtherComp :type Primitive%20Component%20Object%20Reference) (OtherBodyIndex :type Integer))
  (if (not (Collision|IsOverlappingActor OverlappedComponent (Pawn|GetControlledPawn (Variables|Default|GetPlayerControllerREF)) :!class /Script/Engine.PrimitiveComponent))
    (Widget|RemovefromParent (Variables|/Game/Blueprints/Gameplay/GameplayPC.GameplayPC_C|GetShopMenuWB (Variables|Default|GetPlayerControllerREF)))))

(event EventBeginPlay
  (Utilities|FlowControl|Delay 0.2)
  (bind _asgameplay_pc (Utilities|Casting|CastToGameplayPC (Game|GetPlayerController 0)))
  (Variables|Default|SetPlayerControllerREF _asgameplay_pc))

(fn ConstructionScript)