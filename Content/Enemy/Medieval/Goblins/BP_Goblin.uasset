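; BP_Goblin is a medieval goblin enemy that spawns armed with a sword and shield.
; On BeginPlay it calls its parent, then spawns both items at the right and left hand sockets, passing itself as owning goblin, and snaps them to the mesh.
; Only the sword is stored, as Weapon; Tick just forwards to the parent.
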(event EventTick
  (params (DeltaSeconds :type Float%20%28single-precision%29))
  (|CallParentFunction DeltaSeconds))

(event Collision|EventActorBeginOverlap
  (params (OtherActor :type Actor%20Object%20Reference)))

(event EventBeginPlay
  ;[1 1 1] Weapon Attachment
  (|CallParentFunction)
  (Utilities|FlowControl|Sequence
    (:then_0
      (bind _returnvalue (Game|SpawnActorfromClass "/Game/Enemy/Medieval/Goblins/Models/Sword/Goblin_Sword.Goblin_Sword_C" (Transformation|GetSocketTransform (Variables|Character|GetMesh) "hand_R_jntSocket" "RTS_World") "Undefined" 0 self 0.0 0))
      (bind _output_get (Variables|Default|SetWeapon _returnvalue))
      (Transformation|AttachComponentToComponent _output_get (Variables|Character|GetMesh) "hand_R_jntSocket" "SnapToTarget" "SnapToTarget" "SnapToTarget" true))
    (:then_1
      (bind _returnvalue_2 (Game|SpawnActorfromClass "/Game/Enemy/Medieval/Goblins/Models/Shield/Goblin_Shield.Goblin_Shield_C" (Transformation|GetSocketTransform (Variables|Character|GetMesh) "hand_L_jntSocket" "RTS_World") "Undefined" 0 self 0))
      (Transformation|AttachComponentToComponent _returnvalue_2 (Variables|Character|GetMesh) "hand_L_jntSocket" "SnapToTarget" "SnapToTarget" "SnapToTarget" true))))

(fn ConstructionScript)