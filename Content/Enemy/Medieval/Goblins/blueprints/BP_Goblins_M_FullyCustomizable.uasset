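; Customizable male medieval goblin enemy Blueprint with modular clothing, armor, sword and shield.
; The construction script slaves the clothing and armor skeletal meshes to the GoblinsM body via master pose, so they share one animation.
; Per-part Show booleans then toggle visibility of each piece, weapon and shield, configuring each instance's look.
; The event graph holds only disabled placeholder events, so it adds no runtime logic.
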(event EventBeginPlay)

(event Collision|EventActorBeginOverlap
  (params (OtherActor :type Actor%20Object%20Reference)))

(event EventTick
  (params (DeltaSeconds :type Float%20%28single-precision%29)))

(fn ConstructionScript
  (Class|SkinnedMeshComponent|SetMasterPoseComponent (Variables|Default|GetSM_Cloth1_M) (Variables|Default|GetGoblins_M) false)
  (Rendering|SetVisibility (Variables|Default|GetSM_Belt) (Variables|TorsoAndHead|GetShowBelt) false)
  (Rendering|SetVisibility (Variables|Default|GetSM_Cloth1_M) (Variables|TorsoAndHead|GetShowCloth1) false)
  (Rendering|SetVisibility (Variables|Default|GetSM_Cloth2_M) (Variables|TorsoAndHead|GetShowCloth2) false)
  (Rendering|SetVisibility (Variables|Default|GetSM_Collar) (Variables|TorsoAndHead|GetShowCollar) false)
  (Rendering|SetVisibility (Variables|Default|GetSM_Glove_L) (Variables|LeftArm|GetShowGloveL) false)
  (Rendering|SetVisibility (Variables|Default|GetSM_Glove_R) (Variables|RightArm|GetShowGloveR) false)
  (Rendering|SetVisibility (Variables|Default|GetSM_Helmet) (Variables|TorsoAndHead|GetShowHelmet) false)
  (Rendering|SetVisibility (Variables|Default|GetSM_Knee_L_armor) (Variables|LeftLeg|GetShowKneeLArmor) false)
  (Rendering|SetVisibility (Variables|Default|GetSM_Knee_R_armor) (Variables|RightLeg|GetShowKneeRArmor) false)
  (Rendering|SetVisibility (Variables|Default|GetSM_paudron_L) (Variables|LeftArm|GetShowPaudronL) false)
  (Rendering|SetVisibility (Variables|Default|GetSM_paudron_R) (Variables|RightArm|GetShowPaudronR) false)
  (Rendering|SetVisibility (Variables|Default|GetSM_shoe_L) (Variables|LeftLeg|GetShowShoeL) false)
  (Rendering|SetVisibility (Variables|Default|GetSM_shoe_L_armor) (Variables|LeftLeg|GetShowShoeLArmor) false)
  (Rendering|SetVisibility (Variables|Default|GetSM_shoe_R) (Variables|RightLeg|GetShowShowR) false)
  (Rendering|SetVisibility (Variables|Default|GetSM_shoe_R_armor) (Variables|RightLeg|GetShowShoeRArmor) false)
  (Rendering|SetVisibility (Variables|Default|GetSM_shoulder_L_armor) (Variables|LeftArm|GetShowShoulderLArmor) false)
  (Rendering|SetVisibility (Variables|Default|GetSM_shoulder_R_armor) (Variables|RightArm|GetShowShoulderRArmor) false)
  (Rendering|SetVisibility (Variables|Default|GetSM_Skirt) (Variables|TorsoAndHead|GetShowSkirt) false)
  (Rendering|SetVisibility (Variables|Default|GetSM_Chest_armor_M) (Variables|TorsoAndHead|GetShowChestArmor) false)
  (Rendering|SetVisibility (Variables|Default|GetGoblin_Sword) (Variables|Equipment|GetShowWeapon) false)
  (Rendering|SetVisibility (Variables|Default|GetGoblin_Shield1) (Variables|Equipment|GetShowShield) false))