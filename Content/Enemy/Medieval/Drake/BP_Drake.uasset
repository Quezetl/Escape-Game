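; Drake enemy Blueprint that extends a parent enemy with timed attack logic and melee hit checks.
; AttackPlayer uses delays and a DoOnce to open a brief CanCast2nd window, then resets after a cooldown.
; MouthAttack and HandAttack pass jaw or hand socket locations and a GAS damage effect to the parent's CanDamage.
; Overlap and SetByCaller damage helpers are uncalled here, and older trace-attack and blackboard detection chains are disconnected.
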(event Custom|HandAttack
  (CallFunction|CanDamage (Transformation|GetSocketLocation (Variables|Character|GetMesh) "R_Hand") 7e+01 "/Game/Enemy/Oriental/YoungDragon/SecondAttack/YBGE_SADamage.YBGE_SADamage_C" 1e+01 "(TagName=\"Oriental.Enemy.YoungDragon.Ability.SecondAttack.Damage\")"))

(event Custom|MouthAttack
  (CallFunction|CanDamage (Transformation|GetSocketLocation (Variables|Character|GetMesh) "Jaw03") 5e+01 "/Game/Enemy/Oriental/YoungDragon/SecondAttack/YBGE_SADamage.YBGE_SADamage_C" 1e+01 "(TagName=\"Oriental.Enemy.YoungDragon.Ability.SecondAttack.Damage\")"))

(event EventBeginPlay
  (|CallParentFunction))

(event Collision|EventActorBeginOverlap
  (params (OtherActor :type Actor%20Object%20Reference)))

(event EventTick
  (params (DeltaSeconds :type Float%20%28single-precision%29))
  (|CallParentFunction DeltaSeconds))

(event EventAttackPlayer
  (Utilities|FlowControl|Delay 2.0)
  (Utilities|FlowControl|DoOnce false :!label _label
    (:Completed
      (Utilities|FlowControl|Delay 2.0)
      (Variables|Default|SetCanCast2nd true)
      (Utilities|FlowControl|Delay 1.2)
      (Variables|Default|SetCanCast2nd false)
      (Utilities|FlowControl|Delay 5.0)
      (goto _label Reset))))

(event EventCanDamage
  (params (Loc :type Vector :default "0, 0, 0") (Radius :type Float%20%28double-precision%29) (GE :type Gameplay%20Effect%20Class%20Reference) (Damage :type Float%20%28double-precision%29) (Tag :type Gameplay%20Tag%20Structure))
  (|CallParentFunction Loc Radius GE Damage Tag))

(fn ConstructionScript)

(fn CheckOverlap
  (params (MeshLocation :type Vector) (Radius :type Float%20%28double-precision%29))
  (bind _player (Variables|Default|GetPlayer))
  (Utilities|IsValid _player
    (:Is%20Valid
      (bind _returnvalue (Class|PrimitiveComponent|SphereOverlapComponent (Variables|/Script/Engine.Character|GetCapsuleComponent _player) MeshLocation Radius true true true))
      (return _returnvalue))))

(fn AbilityDamage0
  (params (GameplayEffect :type Gameplay%20Effect%20Class%20Reference) (Tag :type Gameplay%20Tag%20Structure))
  (bind _returnvalue (Ability|GameplayEffect|AssignTagSetbyCallerMagnitude (GameplayEffects|MakeOutgoingSpec :self (Variables|Default|GetAbilitySystemComponent) :GameplayEffectClass GameplayEffect) Tag -1e+01))
  (GameplayEffects|ApplyGameplayEffectSpecToTarget (Variables|Default|GetAbilitySystemComponent) _returnvalue (Ability|GetAbilitySystemComponent (Variables|Default|GetPlayer))))