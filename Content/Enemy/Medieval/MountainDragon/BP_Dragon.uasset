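; Mountain Dragon enemy character built on GAS that fights the player with claw and flame abilities and dies at zero health.
; Landing overlap captures the player, while pawn sensing sets the blackboard detection flag.
; Tick updates state booleans from range and health, including a one-time timed flying-attack sequence at 75% health.
; AttackPlayer chains abilities with delays, and Damage applies a SetByCaller effect when a socket sphere overlaps the player's capsule.
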(event OnComponentBeginOverlap(LandingSphere)
  (params (OverlappedComponent :type Primitive%20Component%20Object%20Reference) (OtherActor :type Actor%20Object%20Reference) (OtherComp :type Primitive%20Component%20Object%20Reference) (OtherBodyIndex :type Integer) (bFromSweep :type Boolean) (SweepResult :type Hit%20Result%20Structure%20%28by%20ref%29))
  (bind _asgascharacter (Utilities|Casting|CastToGASCharacter OtherActor))
  (Variables|Default|SetPlayer _asgascharacter)
  (Variables|Animation|SetIsLanding true))

(event OnSeePawn(PawnSensing)
  (params (Pawn :type Pawn%20Object%20Reference))
  (bind _self self)
  (bind _returnvalue (AI|GetAIController _self))
  (bind _returnvalue_2 (AI|GetBlackboard _returnvalue))
  (Utilities|Casting|CastToGASCharacter Pawn)
  (Utilities|IsValid _returnvalue_2
    (:Is%20Valid
      (AI|Components|Blackboard|SetValueasBool _returnvalue_2 (Utilities|Name|MakeLiteralName "detectPlayer") true))))

(event Custom|Attack%20Player
  (Variables|Animation|SetIsAttacking true)
  (Utilities|FlowControl|Delay 2.0)
  (Utilities|FlowControl|DoOnce false :!label _label
    (:Completed
      (Utilities|FlowControl|Delay 1.0)
      (bind _returnvalue (Abilities|TryActivateAbilitybyClass (Variables|Default|GetAbilitySystemComponent) "/Game/Enemy/Medieval/MountainDragon/Abilities/ClawAttack/MDGA_ClawAttack.MDGA_ClawAttack_C" true))
      (Variables|Animation|SetCanCast2nd _returnvalue)
      (Utilities|FlowControl|Delay 1.0)
      (Variables|Animation|SetCanCast2nd false)
      (Utilities|FlowControl|Delay 5.0)
      (bind _returnvalue_2 (Abilities|TryActivateAbilitybyClass (Variables|Default|GetAbilitySystemComponent) "/Game/Enemy/Medieval/MountainDragon/Abilities/FlameAttack/MDGA_FlameAttack.MDGA_FlameAttack_C" true))
      (Variables|Animation|SetCanCast3rd _returnvalue_2)
      (Utilities|FlowControl|Delay 4.33)
      (Variables|Animation|SetCanCast3rd false)
      (goto _label Reset))))

(event Custom|Damage
  (params (Radius :type Float%20%28double-precision%29) (SocketName :type Name) (GE :type Gameplay%20Effect%20Class%20Reference) (Tag :type Gameplay%20Tag%20Structure))
  (Variables|Default|SetSocket%20Name SocketName)
  (bind _result (CallFunction|CheckOverlap (Transformation|GetSocketLocation (Variables|Character|GetMesh) (Variables|Default|GetSocket%20Name)) Radius))
  (if _result
    (CallFunction|AbilityDamage GE Tag)))

(event EventBeginPlay
  (Pawn|Components|CharacterMovement|SetMovementMode (Variables|Character|GetCharacterMovement) "MOVE_Flying" 0))

(event EventTick
  (params (DeltaSeconds :type Float%20%28single-precision%29))
  (bind _player (Variables|Default|GetPlayer))
  (Variables|Default|SetMaxHealth (.ReturnValue (Ability|Attribute|GetFloatAttributefromAbilitySystemComponent (Variables|Default|GetAbilitySystemComponent) "(AttributeName=\"MaxHealth\",Attribute=/Script/Escape_Game.GASAttributeSet:MaxHealth,AttributeOwner=Class'\"/Script/Escape_Game.GASAttributeSet\"')")))
  (bind _output_get (Variables|Default|SetHealth (.ReturnValue (Ability|Attribute|GetFloatAttributefromAbilitySystemComponent (Variables|Default|GetAbilitySystemComponent) "(AttributeName=\"Health\",Attribute=/Script/Escape_Game.GASAttributeSet:Health,AttributeOwner=Class'\"/Script/Escape_Game.GASAttributeSet\"')"))))
  (if (<= _output_get 0.0)
    (Utilities|FlowControl|DoOnce false
      (:Completed
        (Variables|Animation|SetIsDead true)
        (Utilities|FlowControl|Delay 3.0)
        (Actor|DestroyActor)))
    (else
      (Variables|Animation|SetIsDead false)
      (Utilities|IsValid _player
        (:Is%20Valid
          (Math|Float|CompareFloat (Math|Vector|Distance(Vector) (Transformation|GetActorLocation _player) (Transformation|GetActorLocation)) (Variables|Default|GetAttack_Range)
            (:>
              (Variables|Animation|SetIsAttacking false :!label _label))
            (:==
              (goto _label))
            (:<
              (Variables|Animation|SetIsAttacking true)))
          (if (<= (* (/ (Variables|Default|GetHealth) (Variables|Default|GetMaxHealth)) 1e+02) 75.0)
            (if (not (Variables|Animation|GetAnimationLock))
              (Utilities|FlowControl|DoOnce false
                (:Completed
                  (Variables|Animation|SetTakingOff true)
                  (Utilities|FlowControl|Delay 2.3)
                  (Variables|Animation|SetFlyingIdle true)
                  (Utilities|FlowControl|Delay 2.0)
                  (Variables|Animation|SetFlyingAttack true)
                  (Utilities|FlowControl|Delay 8.1)
                  (Variables|Animation|SetFlyingAttack false)
                  (Utilities|FlowControl|Delay 2.0)
                  (Variables|Animation|SetFlyingIdle false)
                  (Utilities|FlowControl|Delay 2.3)
                  (Variables|Animation|SetTakingOff false))))))))))

(fn ConstructionScript)

(fn CheckOverlap
  (params (MeshLocation :type Vector) (Radius :type Float%20%28double-precision%29))
  (bind _player (Variables|Default|GetPlayer))
  (Utilities|IsValid _player
    (:Is%20Valid
      (bind _returnvalue (Class|PrimitiveComponent|SphereOverlapComponent (Variables|/Script/Engine.Character|GetCapsuleComponent _player) MeshLocation Radius true true true))
      (return _returnvalue))))

(fn AbilityDamage
  (params (GameplayEffect :type Gameplay%20Effect%20Class%20Reference) (Tag :type Gameplay%20Tag%20Structure))
  (bind _returnvalue (Ability|GameplayEffect|AssignTagSetbyCallerMagnitude (GameplayEffects|MakeOutgoingSpec :self (Variables|Default|GetAbilitySystemComponent) :GameplayEffectClass GameplayEffect) Tag -1e+01))
  (GameplayEffects|ApplyGameplayEffectSpecToTarget (Variables|Default|GetAbilitySystemComponent) _returnvalue (Ability|GetAbilitySystemComponent (Variables|Default|GetPlayer))))