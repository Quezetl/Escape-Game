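; Griffon enemy Blueprint that extends a parent enemy class with a random flying or ground stance and claw attacks.
; On BeginPlay a random MultiGate flags it as flying or ground, though both branches set movement mode to Flying.
; Attack events feed hand socket locations into the parent's CanDamage with a GameplayEffect and tag, using full damage percent for the ground hit and half for each flying hand.
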(event Custom|GroundAttack
  (CallFunction|CanDamage (Transformation|GetSocketLocation (Variables|Character|GetMesh) "GRIFFON_-L-Hand") 3e+01 "/Game/Enemy/Medieval/Griffon/GFGE_MADamage.GFGE_MADamage_C" 1e+02 "(TagName=\"Medieval.Enemy.Griffon.Ability.MainAttack.Damage\")" "(AttributeName=\"BaseAttackDamage\",Attribute=/Script/Escape_Game.GASAttributeSet:BaseAttackDamage,AttributeOwner=Class'\"/Script/Escape_Game.GASAttributeSet\"')"))

(event Custom|FlyingRightDamage
  (CallFunction|CanDamage (Transformation|GetSocketLocation (Variables|Character|GetMesh) "GRIFFON_-R-Hand") 3e+01 "/Game/Enemy/Medieval/Griffon/GFGE_MADamage.GFGE_MADamage_C" 5e+01 "(TagName=\"Medieval.Enemy.Griffon.Ability.MainAttack.Damage\")" "(AttributeName=\"BaseAttackDamage\",Attribute=/Script/Escape_Game.GASAttributeSet:BaseAttackDamage,AttributeOwner=Class'\"/Script/Escape_Game.GASAttributeSet\"')"))

(event Custom|FlyingLeftDamage
  (CallFunction|CanDamage (Transformation|GetSocketLocation (Variables|Character|GetMesh) "GRIFFON_-L-Hand") 3e+01 "/Game/Enemy/Medieval/Griffon/GFGE_MADamage.GFGE_MADamage_C" 5e+01 "(TagName=\"Medieval.Enemy.Griffon.Ability.MainAttack.Damage\")" "(AttributeName=\"BaseAttackDamage\",Attribute=/Script/Escape_Game.GASAttributeSet:BaseAttackDamage,AttributeOwner=Class'\"/Script/Escape_Game.GASAttributeSet\"')"))

(event EventBeginPlay
  (|CallParentFunction)
  (Utilities|FlowControl|MultiGate true false -1
    (:Out%200
      (Variables|Default|SetIsFlying true)
      (Pawn|Components|CharacterMovement|SetMovementMode (Variables|Character|GetCharacterMovement) "MOVE_Flying" 0))
    (:Out%201
      (Variables|Default|SetIsGround true)
      (Pawn|Components|CharacterMovement|SetMovementMode (Variables|Character|GetCharacterMovement) "MOVE_Flying" 0))))

(event EventDetectPlayer
  (params (Pawn :type Pawn%20Object%20Reference))
  (|CallParentFunction Pawn))

(event EventAttackPlayer
  (|CallParentFunction))

(event EventTick
  (params (DeltaSeconds :type Float%20%28single-precision%29))
  (|CallParentFunction DeltaSeconds))

(event EventCanDamage
  (params (Loc :type Vector :default "0, 0, 0") (Radius :type Float%20%28double-precision%29) (GE :type Gameplay%20Effect%20Class%20Reference) (Percent :type Float%20%28double-precision%29) (Tag :type Gameplay%20Tag%20Structure) (Attribute :type Gameplay%20Attribute%20Structure))
  (|CallParentFunction Loc Radius GE Percent Tag Attribute))

(fn ConstructionScript)