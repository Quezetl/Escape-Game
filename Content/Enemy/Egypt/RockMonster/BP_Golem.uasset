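; Egypt rock golem enemy that damages the player through Gameplay Ability System effects.
; Left-hand, right-hand and clap attack events pass bone locations, effects and tags to the parent CanDamage logic.
; AttackPlayer uses delays and a DoOnce to open a timed CanCast2nd window, then reset.
; Helper functions provide a debug-drawn sphere overlap against the player's capsule and apply tagged, fixed-magnitude SetByCaller damage.
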(event Custom|ClapAttack
  (CallFunction|CanDamage (Transformation|GetSocketLocation (Variables|Character|GetMesh) "Bone056") 5e+01 "/Game/Enemy/Egypt/RockMonster/Abilities/ClapAttack/GLGE_CADamage.GLGE_CADamage_C" 1e+01 "(TagName=\"Egypt.Enemy.Golem.Ability.ClapAttack.Damage\")"))

(event Custom|RightHandAttack
  (CallFunction|CanDamage (Transformation|GetSocketLocation (Variables|Character|GetMesh) "Bone047") 5e+01 "/Game/Enemy/Egypt/RockMonster/Abilities/MainAttack/GLGE_MADamage.GLGE_MADamage_C" 1e+01 "(TagName=\"Egypt.Enemy.Golem.Ability.MainAttack.Damage\")"))

(event Custom|LeftHandAttack
  (CallFunction|CanDamage (Transformation|GetSocketLocation (Variables|Character|GetMesh) "Bone056") 5e+01 "/Game/Enemy/Egypt/RockMonster/Abilities/MainAttack/GLGE_MADamage.GLGE_MADamage_C" 1e+01 "(TagName=\"Egypt.Enemy.Golem.Ability.MainAttack.Damage\")"))

(event Custom|Damage
  (params (Radius :type Float%20%28double-precision%29) (SocketName :type Name) (GE :type Gameplay%20Effect%20Class%20Reference) (Tag :type Gameplay%20Tag%20Structure)))

(event EventBeginPlay)

(event Collision|EventActorBeginOverlap
  (params (OtherActor :type Actor%20Object%20Reference)))

(event EventTick
  (params (DeltaSeconds :type Float%20%28single-precision%29)))

(event EventAttackPlayer
  (Utilities|FlowControl|Delay 2.0)
  (Utilities|FlowControl|DoOnce false :!label _label
    (:Completed
      (Utilities|FlowControl|Delay 4.0)
      (Variables|Default|SetCanCast2nd true)
      (Utilities|FlowControl|Delay 2.4)
      (Variables|Default|SetCanCast2nd false)
      (Utilities|FlowControl|Delay 8.0)
      (goto _label Reset))))

(event EventCanDamage
  (params (Loc :type Vector :default "0, 0, 0") (Radius :type Float%20%28double-precision%29) (GE :type Gameplay%20Effect%20Class%20Reference) (Damage :type Float%20%28double-precision%29) (Tag :type Gameplay%20Tag%20Structure))
  (|CallParentFunction Loc Radius GE Damage Tag))

(fn ConstructionScript)

(fn CheckOverlap
  (params (MeshLocation :type Vector) (Radius :type Float%20%28double-precision%29))
  (bind _player (Variables|Default|GetPlayer))
  (Utilities|IsValid _player
    (:Is%20Valid
      (bind _returnvalue (Class|PrimitiveComponent|SphereOverlapComponent (Variables|/Script/Engine.Character|GetCapsuleComponent _player) MeshLocation Radius true true true))
      (return _returnvalue))))

(fn AbilityDamage
  (params (GameplayEffect :type Gameplay%20Effect%20Class%20Reference) (Tag :type Gameplay%20Tag%20Structure))
  (bind _returnvalue (Ability|GameplayEffect|AssignTagSetbyCallerMagnitude (GameplayEffects|MakeOutgoingSpec :self (Variables|Default|GetAbilitySystemComponent) :GameplayEffectClass GameplayEffect) Tag -1e+01))
  (GameplayEffects|ApplyGameplayEffectSpecToTarget (Variables|Default|GetAbilitySystemComponent) _returnvalue (Ability|GetAbilitySystemComponent (Variables|Default|GetPlayer))))