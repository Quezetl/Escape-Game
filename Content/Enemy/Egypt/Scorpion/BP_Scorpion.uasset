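; BP_Scorpion is the scorpion enemy for the Egypt set, a child Blueprint that leaves detection and attack behavior to its parent.
; Its events forward to the parent, with CanDamage supplying the right claw socket location and a radius for the damage check.
; Unconnected leftover graphs hold older detection, health widget, Gameplay Ability System damage and death logic that never runs.
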(event EventBeginPlay
  (|CallParentFunction))

(event EventTick
  (params (DeltaSeconds :type Float%20%28single-precision%29))
  (|CallParentFunction DeltaSeconds))

(event EventCanDamage
  (params (Loc :type Vector :default "0, 0, 0") (Radius :type Float%20%28double-precision%29))
  (|CallParentFunction (Transformation|GetSocketLocation (Variables|Character|GetMesh) "R_clawJNT5") 3e+01))

(event EventAttackPlayer
  (|CallParentFunction))

(event EventDetectPlayer
  (params (Pawn :type Pawn%20Object%20Reference))
  (|CallParentFunction Pawn))

(fn ConstructionScript)