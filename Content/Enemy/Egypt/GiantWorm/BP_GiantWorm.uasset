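; Giant worm enemy for the Egypt area that stays immobile until a player triggers its appearance.
; BeginPlay disables movement; a GASCharacter entering AppearTrigger sets NotHidden, then after a short delay sets IsAppeared.
; It then writes detectPlayer to the AI controller's Blackboard and restores walking movement.
; AttackPlayer is an empty event, and PawnSensing is unused.
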(event OnComponentBeginOverlap(AppearTrigger)
  (params (OverlappedComponent :type Primitive%20Component%20Object%20Reference) (OtherActor :type Actor%20Object%20Reference) (OtherComp :type Primitive%20Component%20Object%20Reference) (OtherBodyIndex :type Integer) (bFromSweep :type Boolean) (SweepResult :type Hit%20Result%20Structure%20%28by%20ref%29))
  (Utilities|Casting|CastToGASCharacter OtherActor)
  (Development|PrintString "Colliding with player")
  (Variables|Default|SetNotHidden true)
  (Utilities|FlowControl|Delay 2.5)
  (bind _output_get (Variables|Default|SetIsAppeared true))
  (AI|Components|Blackboard|SetValueasBool (AI|GetBlackboard (AI|GetAIController self)) (Utilities|Name|MakeLiteralName "detectPlayer") _output_get)
  (Pawn|Components|CharacterMovement|SetMovementMode (Variables|Character|GetCharacterMovement) "MOVE_Walking" 0))

(event Custom|Attack%20Player)

(event EventBeginPlay
  (Pawn|Components|CharacterMovement|SetMovementMode (Variables|Character|GetCharacterMovement) "MOVE_None" 0))

(event Collision|EventActorBeginOverlap
  (params (OtherActor :type Actor%20Object%20Reference)))

(event EventTick
  (params (DeltaSeconds :type Float%20%28single-precision%29)))

(fn ConstructionScript)