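; Bone dragon enemy for the Egypt area, extending a parent enemy class and using the Gameplay Ability System.
; A sphere overlap stores the player and wakes it, then AttackPlayer cycles wing and flame abilities on timed delays unless taking off.
; Dropping to 75% health triggers a one-time flight sequence driven by timed state flags.
; Jaw and wing-claw events pass socket locations and GameplayEffects to the parent's CanDamage.
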(event OnComponentBeginOverlap(Sphere_0)
  (params (OverlappedComponent :type Primitive%20Component%20Object%20Reference) (OtherActor :type Actor%20Object%20Reference) (OtherComp :type Primitive%20Component%20Object%20Reference) (OtherBodyIndex :type Integer) (bFromSweep :type Boolean) (SweepResult :type Hit%20Result%20Structure%20%28by%20ref%29))
  (bind _asgascharacter (Utilities|Casting|CastToGASCharacter OtherActor))
  (Variables|Default|SetPlayer _asgascharacter)
  (Variables|Default|SetIsAwake true))

(event Custom|WingLeft
  (CallFunction|CanDamage (Transformation|GetSocketLocation (Variables|Character|GetMesh) "WingClaw2_L") 5e+01 "/Game/Enemy/Egypt/BoneDragon/WingAttack/DTGE_WADamage.DTGE_WADamage_C" 1e+01 "(TagName=\"Egypt.Enemy.DemonTerror.Ability.WingAttack.Damage\")"))

(event Custom|MouthDamage
  (CallFunction|CanDamage (Transformation|GetSocketLocation (Variables|Character|GetMesh) "Jaw3") 4e+01 "/Game/Enemy/Egypt/BoneDragon/MouthAttack/DTGE_MADamage.DTGE_MADamage_C" 1e+01 "(TagName=\"Egypt.Enemy.DemonTerror.Ability.MouthAttack.Damage\")"))

(event Custom|WingRight
  (CallFunction|CanDamage (Transformation|GetSocketLocation (Variables|Character|GetMesh) "WingClaw2_R") 5e+01 "/Game/Enemy/Egypt/BoneDragon/WingAttack/DTGE_WADamage.DTGE_WADamage_C" 1e+01 "(TagName=\"Egypt.Enemy.DemonTerror.Ability.WingAttack.Damage\")"))

(event EventBeginPlay
  (|CallParentFunction)
  (Pawn|Components|CharacterMovement|SetMovementMode (Variables|Character|GetCharacterMovement) "MOVE_None" 0))

(event Collision|EventActorBeginOverlap
  (params (OtherActor :type Actor%20Object%20Reference)))

(event EventCanDamage
  (params (Loc :type Vector :default "0, 0, 0") (Radius :type Float%20%28double-precision%29) (GE :type Gameplay%20Effect%20Class%20Reference) (Percent :type Float%20%28double-precision%29) (Tag :type Gameplay%20Tag%20Structure) (Attribute :type Gameplay%20Attribute%20Structure))
  (|CallParentFunction Loc Radius GE Percent Tag Attribute))

(event EventTick
  (params (DeltaSeconds :type Float%20%28single-precision%29))
  (Variables|Default|SetHealth (.ReturnValue (Ability|Attribute|GetFloatAttributefromAbilitySystemComponent (Variables|Default|GetAbilitySystemComponent) "(AttributeName=\"Health\",Attribute=/Script/Escape_Game.GASAttributeSet:Health,AttributeOwner=Class'\"/Script/Escape_Game.GASAttributeSet\"')")))
  (Variables|Default|SetMaxHealth (.ReturnValue (Ability|Attribute|GetFloatAttributefromAbilitySystemComponent (Variables|Default|GetAbilitySystemComponent) "(AttributeName=\"MaxHealth\",Attribute=/Script/Escape_Game.GASAttributeSet:MaxHealth,AttributeOwner=Class'\"/Script/Escape_Game.GASAttributeSet\"')")))
  (|CallParentFunction DeltaSeconds)
  (if (<= (* (/ (Variables|Default|GetHealth) (Variables|Default|GetMaxHealth)) 1e+02) 75.0)
    (if (not (Variables|Default|GetAnimationLock))
      (Utilities|FlowControl|DoOnce false
        (:Completed
          (Variables|Default|SetTakingOff true)
          (Utilities|FlowControl|Delay 1.2)
          (Variables|Default|SetFlyingIdle true)
          (Utilities|FlowControl|Delay 2.0)
          (Variables|Default|SetFlyingAttack true)
          (Utilities|FlowControl|Delay 6.0)
          (Variables|Default|SetFlyingAttack false)
          (Utilities|FlowControl|Delay 2.0)
          (Variables|Default|SetFlyingIdle false)
          (Utilities|FlowControl|Delay 2.0)
          (Variables|Default|SetTakingOff false))))))

(event EventAttackPlayer
  (|CallParentFunction)
  (if (not (Variables|Default|GetTakingOff))
    (Utilities|FlowControl|Delay 2.0)
    (Utilities|FlowControl|DoOnce false :!label _label
      (:Completed
        (Utilities|FlowControl|Delay 1.0)
        (bind _returnvalue (Abilities|TryActivateAbilitybyClass (Variables|Default|GetAbilitySystemComponent) "/Game/Enemy/Egypt/BoneDragon/WingAttack/DTGA_WIngAttack.DTGA_WIngAttack_C" true))
        (Variables|Default|SetCanCast2nd _returnvalue)
        (Utilities|FlowControl|Delay 1.4)
        (Variables|Default|SetCanCast2nd false)
        (Utilities|FlowControl|Delay 3.0)
        (bind _returnvalue_2 (Abilities|TryActivateAbilitybyClass (Variables|Default|GetAbilitySystemComponent) "/Game/Enemy/Egypt/BoneDragon/FlameAttack/DTGA_FlameAttack.DTGA_FlameAttack_C" true))
        (Variables|Default|SetCanCast3rd _returnvalue_2)
        (Utilities|FlowControl|Delay 2.5)
        (Variables|Default|SetCanCast3rd false)
        (goto _label Reset)))))

(event EventDetectPlayer
  (params (Pawn :type Pawn%20Object%20Reference))
  (if (not (Variables|Default|GetAnimationLock))
    (|CallParentFunction Pawn)))

(fn ConstructionScript)

(fn CheckOverlap
  (params (MeshLocation :type Vector) (Radius :type Float%20%28double-precision%29))
  (bind _player (Variables|Default|GetPlayer))
  (Utilities|IsValid _player
    (:Is%20Valid
      (bind _returnvalue (Class|PrimitiveComponent|SphereOverlapComponent (Variables|/Script/Engine.Character|GetCapsuleComponent _player) MeshLocation Radius true true true))
      (return _returnvalue))))

(fn AbilityDamage
  (params (GameplayEffect :type Gameplay%20Effect%20Class%20Reference) (Tag :type Gameplay%20Tag%20Structure))
  (bind _returnvalue (Ability|GameplayEffect|AssignTagSetbyCallerMagnitude (GameplayEffects|MakeOutgoingSpec :self (Variables|Default|GetAbilitySystemComponent) :GameplayEffectClass GameplayEffect) Tag -1e+01))
  (GameplayEffects|ApplyGameplayEffectSpecToTarget (Variables|Default|GetAbilitySystemComponent) _returnvalue (Ability|GetAbilitySystemComponent (Variables|Default|GetPlayer))))