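; Nine-tailed fox enemy that detects, attacks and damages the player through the Gameplay Ability System.
; PawnSensing sets the detectPlayer blackboard key for the AI.
; AttackPlayer sphere-traces forward to cache the player, then applies a SetByCaller damage effect if a bone-socket sphere overlaps the capsule while IsAttackReady is false.
; Tick toggles IsAttacking by distance to that player and destroys the fox shortly after health runs out.
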(event OnSeePawn(PawnSensing)
  (params (Pawn :type Pawn%20Object%20Reference))
  ;[0.1557 0.5417 0.2063] Player Detection
  (Utilities|Casting|CastToGASCharacter Pawn)
  (AI|Components|Blackboard|SetValueasBool (AI|GetBlackboard (AI|GetAIController self)) (Utilities|Name|MakeLiteralName "detectPlayer") true))

(event Custom|Attack%20Player
  (bind _returnvalue (Transformation|GetActorLocation))
  ;[1 0.8354 0.4541] Detect Player to Chase and Attack
  (bind (_outhit _returnvalue_2) (Collision|SphereTraceForObjects _returnvalue (+ _returnvalue (* (Math|Vector|GetForwardVector (Transformation|GetActorRotation)) 2.5e+02)) 1.2e+02 (Utilities|Array|MakeArray "ObjectTypeQuery3") false 0 "ForDuration"))
  (if _returnvalue_2
    (bind _asgascharacter (Utilities|Casting|CastToGASCharacter (.HitActor (Collision|BreakHitResult _outhit))))
    ;[1 0.5166 0.2203] Damage the character once they are in range
    (Utilities|IsValid _asgascharacter
      (:Is%20Valid
        (Variables|Default|SetPlayer _asgascharacter)
        (if (not (Variables|Default|GetIsAttackReady))
          (bind _returnvalue_3 (Class|PrimitiveComponent|SphereOverlapComponent (Variables|/Script/Engine.Character|GetCapsuleComponent _asgascharacter) (Transformation|GetSocketLocation (Variables|Character|GetMesh) "Bone055") 1e+01 false false false))
          (if _returnvalue_3
            (bind _returnvalue_4 (Ability|GameplayEffect|AssignTagSetbyCallerMagnitude (GameplayEffects|MakeOutgoingSpec :self (Variables|Default|GetAbilitySystemComponent) :GameplayEffectClass "/Game/GAS/GE_EnemyAttack.GE_EnemyAttack_C") "(TagName=\"Enemy.NormalAttack.damage\")" -1e+01))
            (GameplayEffects|ApplyGameplayEffectSpecToTarget (Variables|Default|GetAbilitySystemComponent) _returnvalue_4 (Ability|GetAbilitySystemComponent _asgascharacter))))))))

(event EventBeginPlay)

(event Collision|EventActorBeginOverlap
  (params (OtherActor :type Actor%20Object%20Reference)))

(event EventTick
  (params (DeltaSeconds :type Float%20%28single-precision%29))
  (bind _player (Variables|Default|GetPlayer))
  (if (<= (.ReturnValue (Ability|Attribute|GetFloatAttributefromAbilitySystemComponent (Variables|Default|GetAbilitySystemComponent) "(AttributeName=\"Health\",Attribute=/Script/Escape_Game.GASAttributeSet:Health,AttributeOwner=Class'\"/Script/Escape_Game.GASAttributeSet\"')")) 0.0)
    ;[0.6408 0.8232 1] Destroy Actor if the health is <= 0
    (Utilities|FlowControl|DoOnce false
      (:Completed
        (Variables|Default|SetisDead true)
        (Utilities|FlowControl|Delay 2.5)
        (Actor|DestroyActor)))
    (else
      ;[0.7396 0.4618 0.4765] Check If the player is in within the attack range
      (Variables|Default|SetisDead false)
      (Utilities|IsValid _player
        (:Is%20Valid
          (Math|Float|CompareFloat (Math|Vector|Distance(Vector) (Transformation|GetActorLocation _player) (Transformation|GetActorLocation)) (Variables|Default|GetAttack_Range)
            (:>
              (Development|PrintString "Not In Range" :!label _label)
              (Variables|Default|SetIsAttacking false))
            (:==
              (goto _label))
            (:<
              (Variables|Default|SetIsAttacking true))))))))

(fn ConstructionScript)

(fn InRange
  (params (PlayerLocation :type Vector) (EnemyLocation :type Vector)))