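; Turtle monk enemy Blueprint that mostly forwards detection, attack and damage logic to its parent class.
; Each tick it passes HandCollision's world location through a server-named event to store SocketLoc, which CanDamage supplies as the hit location to the parent check.
; TurtleDamage relays an explicit location to that same parent check through TurtleDamageClient.
; Hand overlap events are empty, and older detection, damage, death and wander logic is left disconnected.
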(event OnComponentBeginOverlap(HandCollision)
  (params (OverlappedComponent :type Primitive%20Component%20Object%20Reference) (OtherActor :type Actor%20Object%20Reference) (OtherComp :type Primitive%20Component%20Object%20Reference) (OtherBodyIndex :type Integer) (bFromSweep :type Boolean) (SweepResult :type Hit%20Result%20Structure%20%28by%20ref%29)))

(event OnComponentEndOverlap(HandCollision)
  (params (OverlappedComponent :type Primitive%20Component%20Object%20Reference) (OtherActor :type Actor%20Object%20Reference) (OtherComp :type Primitive%20Component%20Object%20Reference) (OtherBodyIndex :type Integer)))

(event Custom|TurtleDamage
  (params (Socket :type Name) (Radius :type Float%20%28double-precision%29) (GE :type Gameplay%20Effect%20Class%20Reference) (Damage :type Float%20%28double-precision%29) (Tag :type Gameplay%20Tag%20Structure) (Loc :type Vector))
  (CallFunction|TurtleDamageClient "None" Radius GE Damage Tag Loc))

(event Custom|TurtleDamageClient
  (params (Socket :type Name) (Radius :type Float%20%28double-precision%29) (GE :type Gameplay%20Effect%20Class%20Reference) (Damage :type Float%20%28double-precision%29) (Tag :type Gameplay%20Tag%20Structure) (Loc :type Vector))
  (|CallParentFunction Socket Radius GE Damage Tag Loc))

(event Custom|SocketLocChanges
  (params (New%20Loc :type Vector))
  (Transformation|SetWorldLocation (Variables|Default|GetHandCollision) New%20Loc false false)
  (Variables|Default|SetSocketLoc New%20Loc))

(event Custom|SocketLocChangesServer
  (params (New%20Loc :type Vector))
  (CallFunction|SocketLocChanges New%20Loc))

(event EventBeginPlay
  (|CallParentFunction))

(event Collision|EventActorBeginOverlap
  (params (OtherActor :type Actor%20Object%20Reference)))

(event EventTick
  (params (DeltaSeconds :type Float%20%28single-precision%29))
  (|CallParentFunction DeltaSeconds)
  (CallFunction|SocketLocChangesServer (Transformation|GetWorldLocation (Variables|Default|GetHandCollision))))

(event EventCanDamage
  (params (Socket :type Name :default "None") (Radius :type Float%20%28double-precision%29) (GE :type Gameplay%20Effect%20Class%20Reference) (Damage :type Float%20%28double-precision%29) (Tag :type Gameplay%20Tag%20Structure) (Loc :type Vector :default "0, 0, 0"))
  (|CallParentFunction "None" Radius GE Damage Tag (Variables|Default|GetSocketLoc)))

(event EventAttackPlayer
  (|CallParentFunction))

(event EventDetectPlayer
  (params (Pawn :type Pawn%20Object%20Reference))
  (|CallParentFunction Pawn))

(fn ConstructionScript)

(fn TryOverlapComponent
  (params (Mesh%20Loc :type Vector :default "0, 0, 0") (Radius :type Float%20%28double-precision%29))
  (bind _result (|CallParentFunction Mesh%20Loc Radius))
  (return _result))

(fn DamagePlayer
  (params (Tag :type Gameplay%20Tag%20Structure) (Damage :type Float%20%28double-precision%29) (CurrPlayer :type GAS%20Character%20Object%20Reference) (GE :type Gameplay%20Effect%20Class%20Reference))
  (|CallParentFunction Tag Damage 0 GE))