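; Young Dragon enemy driven by GAS that flags player sightings on its AI Blackboard and dies after a short delay at zero health.
; AttackPlayer sphere-traces ahead for the player, then tries the Third attack ability, falling back to the Second.
; Attack events record tongue or arm socket locations, test them against the player's capsule, and apply SetByCaller damage effects.
; Main attack damage events exist, but AttackPlayer never activates that ability.
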(event OnSeePawn(PawnSensing)
  (params (Pawn :type Pawn%20Object%20Reference))
  ;[1 1 1] Find Player
  (Utilities|Casting|CastToGASCharacter Pawn)
  (AI|Components|Blackboard|SetValueasBool (AI|GetBlackboard (AI|GetAIController self)) (Utilities|Name|MakeLiteralName "detectPlayer") true))

(event Custom|AttackPlayer
  (bind _returnvalue (Transformation|GetActorLocation))
  ;[0.1091 0.6771 0.4106] Detect player to attack
  (Variables|Default|SetIsAttacking true)
  (bind (_outhit _returnvalue_2) (Collision|SphereTraceForObjects _returnvalue (+ _returnvalue (* (Math|Vector|GetForwardVector (Transformation|GetActorRotation)) 2.5e+02)) 1.2e+02 (Utilities|Array|MakeArray "ObjectTypeQuery3") false 0 "ForDuration"))
  (if _returnvalue_2
    (bind _asgascharacter (Utilities|Casting|CastToGASCharacter (.HitActor (Collision|BreakHitResult _outhit))))
    (Utilities|IsValid _asgascharacter
      (:Is%20Valid
        (Variables|Default|SetPlayer _asgascharacter)
        ;[0.8211 0.2188 1] Cast Skills
        (Utilities|FlowControl|DoOnce false :!label _label
          (:Completed
            (bind _returnvalue_3 (Abilities|TryActivateAbilitybyClass (Variables|Default|GetAbilitySystemComponent) "/Game/Enemy/Oriental/YoungDragon/ThirdAttack/YBGA_ThirdAttack.YBGA_ThirdAttack_C" true))
            (Utilities|FlowControl|Delay 0.8)
            (bind _output_get (Variables|Default|SetCanCast3rd _returnvalue_3))
            (if _output_get
              (goto _label Reset)
              (else
                (bind _returnvalue_4 (Abilities|TryActivateAbilitybyClass (Variables|Default|GetAbilitySystemComponent) "/Game/Enemy/Oriental/YoungDragon/SecondAttack/YBGA_SecondAttack.YBGA_SecondAttack_C" true))
                (Utilities|FlowControl|Delay 1.1)
                (bind _output_get_2 (Variables|Default|SetCanCast2nd _returnvalue_4))
                (if _output_get_2
                  (goto _label Reset)
                  (else
                    (Abilities|TryActivateAbilitybyClass (Variables|Default|GetAbilitySystemComponent) "/Game/Enemy/Oriental/YoungDragon/SecondAttack/YBGA_SecondAttack.YBGA_SecondAttack_C" true)
                    (goto _label Reset)))))))))))

(event Custom|MADamage
  ;[0.3625 1 0.9502] Main Attack Damage
  (bind _result (CallFunction|CheckOverlap (Utilities|Array|Get(acopy) (Variables|Default|GetMASocketLocations)) 2e+01))
  (Utilities|Array|Clear (Variables|Default|GetMASocketLocations))
  (if _result
    (CallFunction|AbilityDamage "/Game/Enemy/Oriental/YoungDragon/MainAttack/YBGE_MADamage.YBGE_MADamage_C" "(TagName=\"Oriental.Enemy.YoungDragon.Ability.MainAttack.Damage\")")))

(event Custom|SAStoreLoc
  ;[0.4591 1 0.2598] Second Attack Damage
  (Utilities|Array|Add (Variables|Default|GetSASocketLocations) (Transformation|GetSocketLocation (Variables|Default|GetYoungDragon_HeadB) "Tongue2")))

(event Custom|TAStoreLoc
  ;[1 0.5208 0.5208] Third Attack Damage
  (Utilities|Array|Add (Variables|Default|GetTASocketLocations) (Transformation|GetSocketLocation (Variables|Character|GetYoungDragon_Rig+Anim) "YoungDragonRArm2")))

(event Custom|TADamage
  ;[1 0.5208 0.5208] Third Attack Damage
  (bind _result (CallFunction|CheckOverlap (Utilities|Array|Get(acopy) (Variables|Default|GetTASocketLocations)) 1.2e+02))
  (Utilities|Array|Clear (Variables|Default|GetTASocketLocations))
  (if _result
    (CallFunction|AbilityDamage "/Game/Enemy/Oriental/YoungDragon/ThirdAttack/YBGE_TADamage.YBGE_TADamage_C" "(TagName=\"Oriental.Enemy.YoungDragon.Ability.ThirdAttack.Damage\")")
    (Development|PrintString "TA Doing Damage")))

(event Custom|SADamage
  ;[0.4591 1 0.2598] Second Attack Damage
  (bind _result (CallFunction|CheckOverlap (Utilities|Array|Get(acopy) (Variables|Default|GetSASocketLocations)) 3e+01))
  (Utilities|Array|Clear (Variables|Default|GetSASocketLocations))
  (if _result
    (CallFunction|AbilityDamage "/Game/Enemy/Oriental/YoungDragon/SecondAttack/YBGE_SADamage.YBGE_SADamage_C" "(TagName=\"Oriental.Enemy.YoungDragon.Ability.SecondAttack.Damage\")")
    (Development|PrintString "SA Doing Damage")))

(event Custom|MAStoreLoc
  ;[0.3625 1 0.9502] Main Attack Damage
  (Utilities|Array|Add (Variables|Default|GetMASocketLocations) (Transformation|GetSocketLocation (Variables|Default|GetYoungDragon_HeadB) "Tongue2")))

(event Custom|CustomEvent)

(event EventBeginPlay)

(event Collision|EventActorBeginOverlap
  (params (OtherActor :type Actor%20Object%20Reference)))

(event EventTick
  (params (DeltaSeconds :type Float%20%28single-precision%29))
  (if (<= (.ReturnValue (Ability|Attribute|GetFloatAttributefromAbilitySystemComponent (Variables|Default|GetAbilitySystemComponent) "(AttributeName=\"Health\",Attribute=/Script/Escape_Game.GASAttributeSet:Health,AttributeOwner=Class'\"/Script/Escape_Game.GASAttributeSet\"')")) 0.0)
    ;[1 0.3733 0.5973] Destroy actor if health <= 0
    (Utilities|FlowControl|DoOnce false
      (:Completed
        (Variables|Default|SetisDead true)
        (Utilities|FlowControl|Delay 2.5)
        (Actor|DestroyActor)))
    (else
      (Variables|Default|SetisDead false))))

(fn ConstructionScript)

(fn CheckOverlap
  (params (MeshLocation :type Vector) (Radius :type Float%20%28double-precision%29))
  (bind _player (Variables|Default|GetPlayer))
  (Utilities|IsValid _player
    (:Is%20Valid
      (bind _returnvalue (Class|PrimitiveComponent|SphereOverlapComponent (Variables|/Script/Engine.Character|GetCapsuleComponent _player) MeshLocation Radius true true true))
      (return _returnvalue))))

(fn AbilityDamage
  (params (GameplayEffect :type Gameplay%20Effect%20Class%20Reference) (Tag :type Gameplay%20Tag%20Structure))
  (bind _returnvalue (Ability|GameplayEffect|AssignTagSetbyCallerMagnitude (GameplayEffects|MakeOutgoingSpec :self (Variables|Default|GetAbilitySystemComponent) :GameplayEffectClass GameplayEffect) Tag -1e+01))
  (GameplayEffects|ApplyGameplayEffectSpecToTarget (Variables|Default|GetAbilitySystemComponent) _returnvalue (Ability|GetAbilitySystemComponent (Variables|Default|GetPlayer))))