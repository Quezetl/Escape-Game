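; Phoenix enemy character that detects and attacks the player using GAS and a Behavior Tree blackboard.
; Pawn sensing sets the detectPlayer key, and AttackPlayer stores the player found by a forward sphere trace.
; Tick sets IsAttacking by range to that player and destroys the enemy after a delay once its attribute is depleted.
; DamageEnemy overlaps spheres at both toe sockets with the player's capsule, applying SetByCaller damage on contact.
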(event OnSeePawn(PawnSensing)
  (params (Pawn :type Pawn%20Object%20Reference))
  (Utilities|Casting|CastToGASCharacter Pawn)
  (AI|Components|Blackboard|SetValueasBool (AI|GetBlackboard (AI|GetAIController self)) (Utilities|Name|MakeLiteralName "detectPlayer") true))

(event Custom|Attack%20Player
  (bind _returnvalue (Transformation|GetActorLocation))
  (bind (_outhit _returnvalue_2) (Collision|SphereTraceForObjects _returnvalue (+ _returnvalue (* (Math|Vector|GetForwardVector (Transformation|GetActorRotation)) 2.5e+02)) 1.2e+02 (Utilities|Array|MakeArray "ObjectTypeQuery3") false 0 "ForDuration"))
  (if _returnvalue_2
    (bind _asgascharacter (Utilities|Casting|CastToGASCharacter (.HitActor (Collision|BreakHitResult _outhit))))
    (Utilities|IsValid _asgascharacter
      (:Is%20Valid
        (Variables|Default|SetPlayer _asgascharacter)))))

(event Custom|Damage%20Enemy
  (bind _returnvalue (Class|PrimitiveComponent|SphereOverlapComponent (Variables|/Script/Engine.Character|GetCapsuleComponent (Variables|Default|GetPlayer)) (Transformation|GetSocketLocation (Variables|Character|GetMesh) "J_tumasaki_R") 4e+01 true true true))
  (bind _returnvalue_2 (Class|PrimitiveComponent|SphereOverlapComponent (Variables|/Script/Engine.Character|GetCapsuleComponent (Variables|Default|GetPlayer)) (Transformation|GetSocketLocation (Variables|Character|GetMesh) "J_tumasaki_L") 4e+01 true true true))
  (if (or _returnvalue_2 _returnvalue)
    (bind _returnvalue_3 (Ability|GameplayEffect|AssignTagSetbyCallerMagnitude (GameplayEffects|MakeOutgoingSpec :self (Variables|Default|GetAbilitySystemComponent) :GameplayEffectClass "/Game/GAS/GE_EnemyAttack.GE_EnemyAttack_C") "(TagName=\"Enemy.NormalAttack.damage\")" -1e+01))
    (GameplayEffects|ApplyGameplayEffectSpecToTarget (Variables|Default|GetAbilitySystemComponent) _returnvalue_3 (Ability|GetAbilitySystemComponent (Variables|Default|GetPlayer)))))

(event EventBeginPlay)

(event Collision|EventActorBeginOverlap
  (params (OtherActor :type Actor%20Object%20Reference)))

(event EventTick
  (params (DeltaSeconds :type Float%20%28single-precision%29))
  (bind _player (Variables|Default|GetPlayer))
  (if (<= (.ReturnValue (Ability|Attribute|GetFloatAttributefromAbilitySystemComponent (Variables|Default|GetAbilitySystemComponent) "(AttributeName=\"Health\",Attribute=/Script/Escape_Game.GASAttributeSet:Health,AttributeOwner=Class'\"/Script/Escape_Game.GASAttributeSet\"')")) 0.0)
    (Utilities|FlowControl|DoOnce false
      (:Completed
        (Variables|Default|SetisDead true)
        (Utilities|FlowControl|Delay 2.5)
        (Actor|DestroyActor)))
    (else
      (Variables|Default|SetisDead false)
      (Utilities|IsValid _player
        (:Is%20Valid
          (Math|Float|CompareFloat (Math|Vector|Distance(Vector) (Transformation|GetActorLocation _player) (Transformation|GetActorLocation)) (Variables|Default|GetAttack_Range)
            (:>
              (Development|PrintString "Not In Range" :!label _label)
              (Variables|Default|SetIsAttacking false))
            (:==
              (goto _label))
            (:<
              (Variables|Default|SetIsAttacking true))))))))

(fn ConstructionScript)