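; BP_OniWeapon is the Oni enemy's weapon, which deals normal attack damage to the player through the Gameplay Ability System.
; Its Box overlap caches any overlapping GASCharacter as Player, with no code to clear it.
; CanDamage applies GE_EnemyAttack from the Oni's ability system to that Player, passing fixed damage as a tagged SetByCaller magnitude.
; CannotDamage is empty, and the flinch check and DoOnce cooldown are disconnected.
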(event OnComponentBeginOverlap(Box)
  (params (OverlappedComponent :type Primitive%20Component%20Object%20Reference) (OtherActor :type Actor%20Object%20Reference) (OtherComp :type Primitive%20Component%20Object%20Reference) (OtherBodyIndex :type Integer) (bFromSweep :type Boolean) (SweepResult :type Hit%20Result%20Structure%20%28by%20ref%29))
  (bind _asgascharacter (Utilities|Casting|CastToGASCharacter OtherActor))
  (Utilities|IsValid _asgascharacter
    (:Is%20Valid
      (Variables|Default|SetPlayer _asgascharacter))))

(event EventBeginPlay)

(event Collision|EventActorBeginOverlap
  (params (OtherActor :type Actor%20Object%20Reference)))

(event EventTick
  (params (DeltaSeconds :type Float%20%28single-precision%29)))

(event EventCanDamage
  (bind _returnvalue (Ability|GameplayEffect|AssignTagSetbyCallerMagnitude (GameplayEffects|MakeOutgoingSpec :self (Ability|GetAbilitySystemComponent (Variables|Default|GetBP_Oni)) :GameplayEffectClass "/Game/GAS/GE_EnemyAttack.GE_EnemyAttack_C") "(TagName=\"Enemy.NormalAttack.damage\")" -1e+01))
  (GameplayEffects|ApplyGameplayEffectSpecToTarget (Ability|GetAbilitySystemComponent (Variables|Default|GetBP_Oni)) _returnvalue (Ability|GetAbilitySystemComponent (Variables|Default|GetPlayer))))

(event EventCannotDamage)

(fn ConstructionScript)