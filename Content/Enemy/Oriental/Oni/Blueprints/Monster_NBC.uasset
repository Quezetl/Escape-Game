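; Monster AI character built on the MTK toolkit, with Behavior Tree-driven senses, melee and death.
; Sight and cooldown-limited hearing of players write target and status to the Blackboard.
; Point damage reduces health, triggering blood effects or death by ragdoll or random montage through multicast events, with empty MTK hooks for extensions.
; A right-hand sphere damages the current target once per reset, gated by events intended for animation notifies.
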(event OnComponentBeginOverlap(HitSphere)
  (params (OverlappedComponent :type Primitive%20Component%20Object%20Reference) (OtherActor :type Actor%20Object%20Reference) (OtherComp :type Primitive%20Component%20Object%20Reference) (OtherBodyIndex :type Integer) (bFromSweep :type Boolean) (SweepResult :type Hit%20Result%20Structure%20%28by%20ref%29))
  (bind _returnvalue (AI|GetBlackboard 0))
  ;[1 0.08333 0.08333] Note: this damage is not a part of the system it's only for a quick testing or a presentation for  how you can apply damage.
  ;;[1 1 1] Apply Damage when the "Hit Sphere" overlap with an actor and the"Can Apply Damage" is True
  (Utilities|IsValid _returnvalue
    (:Is%20Valid
      (if (and (== OtherActor (AI|Components|Blackboard|GetValueasObject _returnvalue (Utilities|Name|MakeLiteralName "TargetActor"))) (Variables|Default|GetCanApplyDamage?))
        (Utilities|FlowControl|DoOnce false
          (:Completed
            (Game|Damage|ApplyDamage OtherActor (Variables|MonsterKitValues|GetBase%20Damage) 0 self)))))))

(event OnTargetPerceptionUpdated(MTK_AIPerception)
  (params (Actor :type Actor%20Object%20Reference) (Stimulus :type AI%20Stimulus%20Structure))
  ;[1 1 1] Perception
  (CallFunction|MTKPerception Actor Stimulus))

(event Custom|MTK_OnGetDamage
  ;[1 0.7696 0.2474] Monster Ai tool Kit Events - (You can use it if you want to add any features at a specefic event)
)

(event Custom|MTK_OnSight
  ;[1 0.7696 0.2474] Monster Ai tool Kit Events - (You can use it if you want to add any features at a specefic event)
)

(event Custom|MTK_OnAttackFinished
  ;[1 0.7696 0.2474] Monster Ai tool Kit Events - (You can use it if you want to add any features at a specefic event)
)

(event Custom|MTK_OnInvestigateEachRound
  ;[1 0.7696 0.2474] Monster Ai tool Kit Events - (You can use it if you want to add any features at a specefic event)
)

(event Custom|MTK_OnDeadAnimationFinished
  ;[1 0.7696 0.2474] Monster Ai tool Kit Events - (You can use it if you want to add any features at a specefic event)
)

(event Custom|Reset%20Apply%20Damage
  ;[1 0.08333 0.08333] Note: this damage is not a part of the system it's only for a quick testing or a presentation for  how you can apply damage.
  ;;[1 1 1] Apply Damage when the "Hit Sphere" overlap with an actor and the"Can Apply Damage" is True
  ;;;[1 1 1] you can access these Events from "animation notify" to specify which part of Animation is making the damage, and when the animation ends
  (Variables|Default|SetCanApplyDamage? true)
  (Utilities|FlowControl|DoOnce false) ; enters at Reset
)

(event Custom|PlayAnimationMulticast
  (params (AnimMontage :type Anim%20Montage%20Object%20Reference))
  ;[1 1 1] Play MultiCast Animation
  (Animation|PlayAnimMontage AnimMontage 1.0 "None"))

(event Custom|Set%20Apply%20Damage
  ;[1 0.08333 0.08333] Note: this damage is not a part of the system it's only for a quick testing or a presentation for  how you can apply damage.
  ;;[1 1 1] Apply Damage when the "Hit Sphere" overlap with an actor and the"Can Apply Damage" is True
  ;;;[1 1 1] you can access these Events from "animation notify" to specify which part of Animation is making the damage, and when the animation ends
  (Variables|Default|SetCanApplyDamage? true))

(event Custom|PlayEmitterMulticast
  (params (Hit :type Hit%20Result%20Structure%20%28by%20ref%29))
  ;[1 1 1] Play MultiCast Emitter Multiplayer, Used for Blood Effect
  (Effects|SpawnEmitterAttached (Variables|MonsterKit|GetDamageEffect) (Variables|Character|GetMesh) "None" (.ImpactPoint (Collision|BreakHitResult Hit)) "0, 0, 0" "1.000000,1.000000,1.000000" "KeepWorldPosition"))

(event Custom|RagDollMultiCast
  ;[1 1 1] RagDoll, Multicast
  (Physics|SetSimulatePhysics (Variables|Character|GetMesh) true))

(event Custom|DisableAnimationMulticast
  ;[1 1 1] Pause Animation Multicast
  (Class|AnimInstance|MontagePause (Components|SkeletalMesh|GetAnimInstance (Variables|Character|GetMesh)) (Animation|GetCurrentMontage :!class /Script/Engine.Character))
  (Components|Activation|Deactivate (Variables|Character|GetMesh)))

(event Custom|DestroyAiMulticast
  (bind _returnvalue (Pawn|GetController))
  ;[1 1 1] Destroy upon death in Multicast
  (Components|DestroyComponent (Variables|Default|GetMTK_AIPerception))
  (Utilities|IsValid _returnvalue
    (:Is%20Valid
      (Pawn|UnPossess _returnvalue))
    (:Is%20Not%20Valid
      _))
  (Components|DestroyComponent (Variables|Collision|GetCapsuleComponent))
  (Collision|SetCollisionProfileName (Variables|Character|GetMesh) "Ragdoll" true :!class /Script/Engine.PrimitiveComponent)
  (Pawn|Components|CharacterMovement|SetMovementMode (Variables|Character|GetCharacterMovement) "MOVE_None" 0))

(event Custom|MTK_OnHearing
  ;[1 0.7696 0.2474] Monster Ai tool Kit Events - (You can use it if you want to add any features at a specefic event)
)

(event Custom|ResetHearing
  ;[1 1 1] Perception
  ;;[1 1 1] Perception Function will call this Event To prevent Hearing Function From Glitching!
  (Utilities|FlowControl|Delay 2.0)
  (Variables|Default|SetCanSearch? true))

(event Custom|InitiateMonsterAi
  ;[1 1 1] This custom event will run after attaching the behavior tree to make sure the initialization of MonsterAiKit is executing in the right order.
  ;[1 1 1] Initiate Monster Ai Sys
  ;;[1 1 1] Check PatrolLooping Option
  (AI|Components|Blackboard|SetValueasBool (AI|GetBlackboard 0) (Utilities|Name|MakeLiteralName "PatrolLooping?") (Variables|MonsterKit|GetPatrolLooping?))
  ;;[1 1 1] Setup-Init-State
  (AI|Components|Blackboard|SetValueasEnum (AI|GetBlackboard 0) (Utilities|Name|MakeLiteralName "InitialState") (Variables|MonsterKit|GetInitialState))
  ;[1 1 1] Set The Initial SpawnPoint
  (Variables|Default|SetspawnPoint (Transformation|GetActorLocation)))

(event Custom|MTK_OnChaseStart
  ;[1 0.7696 0.2474] Monster Ai tool Kit Events - (You can use it if you want to add any features at a specefic event)
)

(event Custom|MTK_OnLoseSight
  ;[1 0.7696 0.2474] Monster Ai tool Kit Events - (You can use it if you want to add any features at a specefic event)
)

(event Custom|MTK_OnInvestigateStart
  ;[1 0.7696 0.2474] Monster Ai tool Kit Events - (You can use it if you want to add any features at a specefic event)
)

(event Custom|MTK_OnDead
  ;[1 0.7696 0.2474] Monster Ai tool Kit Events - (You can use it if you want to add any features at a specefic event)
)

(event Custom|MTK_OnAttackStart
  ;[1 0.7696 0.2474] Monster Ai tool Kit Events - (You can use it if you want to add any features at a specefic event)
)

(event Game|Damage|EventPointDamage
  (params (Damage :type Float%20%28single-precision%29) (DamageType :type Damage%20Type%20Object%20Reference) (HitLocation :type Vector :default "0, 0, 0") (HitNormal :type Vector :default "0, 0, 0") (HitComponent :type Primitive%20Component%20Object%20Reference) (BoneName :type Name :default "None") (ShotFromDirection :type Vector :default "0, 0, 0") (InstigatedBy :type Controller%20Object%20Reference) (DamageCauser :type Actor%20Object%20Reference) (HitInfo :type Hit%20Result%20Structure%20%28by%20ref%29))
  ;[1 0.651 0.651] Use only one of them(point damage or any damage) don't use the two at the same time!
  ;;[1 1 1] Event Get Any Point Damage (Attach it if you will use point damage event ), point damage make the particle effect of blood works
  (bind (_dead _dyinganimationtime _dieragdoll_) (CallFunction|MTKGetDamage Damage DamageCauser))
  (if _dead
    (Utilities|FlowControl|Delay _dyinganimationtime)
    (CallFunction|MTKFinishDeathAnimation _dieragdoll_)
    (else
      (CallFunction|PlayEmitterMulticast HitInfo))))

(event Game|Damage|EventAnyDamage
  (params (Damage :type Float%20%28single-precision%29) (DamageType :type Damage%20Type%20Object%20Reference) (InstigatedBy :type Controller%20Object%20Reference) (DamageCauser :type Actor%20Object%20Reference))
  ;[1 0.651 0.651] Use only one of them(point damage or any damage) don't use the two at the same time!
  ;;[1 1 1] Event Get Any DamageGet (Attach it if you will use AnyDamage Event)
)

(event EventBeginPlay
  ;[1 0.4681 0.3277] Event Begin Play
  (Utilities|FlowControl|Sequence
    (:then_0
      ;[0.599 0.3209 0.287] Setting Up the damage collision
      (Transformation|AttachComponentToComponent (Variables|Default|GetHit%20Sphere) (Variables|Character|GetMesh) "hand_r" "KeepRelative" "KeepRelative" "KeepRelative" true))))

(fn ConstructionScript)

(fn MTKGetDamage
  (params (Damage :type Float%20%28double-precision%29) (InstigatorActorRef :type Actor%20Object%20Reference))
  (bind _dying_animations (Variables|MonsterKitAnimation|GetDying_Animations))
  (bind _returnvalue (Utilities|Array|Length _dying_animations))
  (bind _returnvalue_2 (Math|Random|RandomInteger _returnvalue))
  (bind _output (Utilities|Array|Get(acopy) _dying_animations _returnvalue_2))
  ;[1 0 0] Get Damage and Death Handling
  (Utilities|IsValid (AI|GetBlackboard 0)
    (:Is%20Valid
      (AI|Components|Blackboard|SetValueasEnum (AI|GetBlackboard 0) (Utilities|Name|MakeLiteralName "Status") (Utilities|Enum|LiteralenumMonsterKitStatus "NewEnumerator3"))
      (Development|PrintString (Utilities|GetDisplayName InstigatorActorRef))
      (bind _healthafterdamage (CallFunction|MTKCalculateHealth Damage))
      (AI|Components|Blackboard|SetValueasVector (AI|GetBlackboard 0) (Utilities|Name|MakeLiteralName "DamageCauserLocation") (Transformation|GetActorLocation InstigatorActorRef))
      ;;[1 1 1] DeathHandling
      (if (<= _healthafterdamage 0.0)
        (if (Utilities|IsValid (Pawn|GetController))
          (CallFunction|DestroyAiMulticast)
          ;;;[1 1 1] Play Dying Animation
          (if (Variables|MonsterKit|GetDieRagDoll?)
            (CallFunction|RagDollMultiCast)
            (CallFunction|MTKonDead)
            (return true 0.0 (Variables|MonsterKit|GetDieRagDoll?))
            (else
              (CallFunction|MTKonDead)
              (CallFunction|PlayAnimationMulticast _output)
              (return true (- (Animation|GetPlayLength _output) 0.5) (Variables|MonsterKit|GetDieRagDoll?)))))
        (else
          (CallFunction|MTKonGetDamage))))))

(fn MTKCalculateHealth
  (params (Damage :type Float%20%28double-precision%29))
  (bind _output_get (Variables|MonsterKit|SetHealth (- (Variables|MonsterKit|GetHealth) Damage)))
  (return _output_get))

(fn MTKAfterDeathAnimation
  (params (AnimMontage :type Anim%20Montage%20Object%20Reference)))

(fn MTKPerception
  (params (Actor :type Actor%20Object%20Reference) (Stimulus :type AI%20Stimulus%20Structure))
  (bind _bsuccessfullysensed (Utilities|Struct|BreakAIStimulus Stimulus))
  (bind _returnvalue (AI|GetBlackboard 0))
  (bind _returnvalue_2 (Game|GetPlayerCharacter 0))
  (bind _returnvalue_3 (Actor|ActorHasTag Actor "player"))
  (bind _returnvalue_4 (AI|GetBlackboard 0))
  (bind _returnvalue_5 (== Actor _returnvalue_2))
  (bind _returnvalue_6 (or _returnvalue_5 _returnvalue_3))
  ;[1 1 1] Vision
  (bind _returnvalue_7 (Class|AIPerceptionSystem|GetSenseClassforStimulus Stimulus))
  (if (== _returnvalue_7 "/Script/AIModule.AISense_Sight")
    (if _returnvalue_6
      (Utilities|IsValid _returnvalue_4
        (:Is%20Valid
          (AI|Components|Blackboard|SetValueasObject _returnvalue_4 (Utilities|Name|MakeLiteralName "TargetActor") Actor)
          (AI|Components|Blackboard|SetValueasBool (AI|GetBlackboard 0) (Utilities|Name|MakeLiteralName "CanSeePlayer?") _bsuccessfullysensed)
          (Utilities|FlowControl|Sequence
            (:then_0
              (if _bsuccessfullysensed
                (AI|Components|Blackboard|SetValueasEnum (AI|GetBlackboard 0) (Utilities|Name|MakeLiteralName "Status") (Utilities|Enum|LiteralenumMonsterKitStatus "NewEnumerator4"))
                (CallFunction|MTKonSight)
                (else
                  (AI|Components|Blackboard|SetValueasEnum (AI|GetBlackboard 0) (Utilities|Name|MakeLiteralName "Status") (Utilities|Enum|LiteralenumMonsterKitStatus "NewEnumerator2"))
                  (CallFunction|MTKonChaseStart))))
            (:then_1
              ;;[1 1 1] Run (OnLoseSightEvent)
              (if (not _bsuccessfullysensed)
                (CallFunction|MTKonLoseSight)))))))
    (else
      ;[1 1 1] Hearing
      (if _returnvalue_6
        (if (not (ScalableFloat|GetValueasBool (AI|GetBlackboard 0) (Utilities|Name|MakeLiteralName "CanSeePlayer?")))
          (AI|Components|Blackboard|SetValueasObject _returnvalue (Utilities|Name|MakeLiteralName "TargetActor") Actor)
          (AI|Components|Blackboard|SetValueasVector _returnvalue (Utilities|Name|MakeLiteralName "TargetLocation") (Transformation|GetActorLocation Actor))
          (if (== (Class|BlackboardComponent|GetValueasEnum (AI|GetBlackboard 0) (Utilities|Name|MakeLiteralName "Status")) (Utilities|Enum|LiteralenumMonsterKitStatus "NewEnumerator1"))
            ;;[1 1 1] Set it first to "Nothing" so it can reset the value everytime it hears the player
            (if (Variables|Default|GetCanSearch?)
              (AI|Components|Blackboard|SetValueasEnum (AI|GetBlackboard 0) (Utilities|Name|MakeLiteralName "Status") (Utilities|Enum|LiteralenumMonsterKitStatus "NewEnumerator5"))
              (AI|Components|Blackboard|SetValueasEnum (AI|GetBlackboard 0) (Utilities|Name|MakeLiteralName "Status") (Utilities|Enum|LiteralenumMonsterKitStatus "NewEnumerator1") :!label _label)
              (Variables|Default|SetCanSearch? false)
              (CallFunction|ResetHearing)
              (CallFunction|MTKonHearing))
            (elif (Variables|Default|GetCanSearch?)
              (goto _label))))))))

(fn MTKFinishDeathAnimation
  (params (DieRagDol? :type Boolean))
  (if DieRagDol?
    _
    (else
      (CallFunction|DisableAnimationMulticast)))
  (CallFunction|MTKonDeadAnimationFinished))