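; Oni enemy character that detects the player, plays an attack montage and dies, using the Gameplay Ability System.
; BeginPlay spawns an Oni weapon onto its hand socket, and pawn sensing sets a blackboard flag when it sees the player character.
; Tick prints and polls an ability-system attribute, setting IsDead and destroying the actor after a delay at zero.
; AttackPlayer only plays the montage; older trace and gameplay-effect damage logic is left disconnected.
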(event OnSeePawn(PawnSensing)
  (params (Pawn :type Pawn%20Object%20Reference))
  ;[1 1 1] Player Detection
  (Utilities|Casting|CastToGAS_Character Pawn)
  (AI|Components|Blackboard|SetValueasBool (AI|GetBlackboard (AI|GetAIController self)) (Utilities|Name|MakeLiteralName "detectPlayer") true))

(event Custom|Attack%20Player
  ;[1 1 1] Chase-Attack
  (Variables|Default|SetisFlinching false)
  (Animation|PlayAnimMontage "/Game/Enemy/Oriental/Oni/Animations/oni_attack_Montage.oni_attack_Montage" 1.0 "None"))

(event EventBeginPlay
  (bind _returnvalue (Game|SpawnActorfromClass "/Game/GASEnemy/BP_OniWeapon.BP_OniWeapon_C" (Transformation|GetSocketTransform (Variables|Character|GetMesh) "WeaponSocket" "RTS_Actor") "Undefined" 0 self false 0))
  (bind _output_get (Variables|Default|SetWeapon _returnvalue))
  (Transformation|AttachComponentToComponent _output_get (Variables|Character|GetMesh) "WeaponSocket" "SnapToTarget" "SnapToTarget" "SnapToTarget" true))

(event Collision|EventActorBeginOverlap
  (params (OtherActor :type Actor%20Object%20Reference)))

(event EventTick
  (params (DeltaSeconds :type Float%20%28single-precision%29))
  (bind _abilitysystemcomponent (Variables|Default|GetAbilitySystemComponent))
  (bind _returnvalue (Ability|Attribute|GetFloatAttributefromAbilitySystemComponent _abilitysystemcomponent "(AttributeName=\"Health\",Attribute=/Script/Escape_Game.GASAttributeSet:Health,AttributeOwner=Class'\"/Script/Escape_Game.GASAttributeSet\"')"))
  (Development|PrintString (Utilities|String|ToString(Float) _returnvalue))
  (if (<= _returnvalue 0.0)
    (Utilities|FlowControl|DoOnce false
      (:Completed
        (Variables|Default|SetisDead true)
        (Utilities|FlowControl|Delay 3.0)
        (Actor|DestroyActor)))
    (else
      (Variables|Default|SetisDead false))))

(fn ConstructionScript)