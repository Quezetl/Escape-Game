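; Raijin boss enemy Blueprint that fights players with meteor and burn attacks through the Gameplay Ability System.
; BeginPlay attaches left and right weapons, and AttackPlayer runs a DoOnce-gated, delay-timed chain of meteor abilities with cast flags.
; Tick triggers a one-time flying phase at 75% health or below, toggling timed state flags.
; Separate events spawn the attack actors at Raijin's hand, the target player, or every GASCharacter.
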(event Custom|SpawnMeteor
  (Game|SpawnActorfromClass "/Game/Enemy/Oriental/Raijin_GodOfThunder/Abilities/SpawnMeteor/BP_SpawnMeteor.BP_SpawnMeteor_C" (Math|Transform|MakeTransform (+ (Transformation|GetSocketLocation (Variables|Character|GetMesh) "weapon_r") "0,0,-40.000000") (Transformation|GetActorRotation self)) "Undefined" 0 self 0))

(event Custom|MeteorAttack
  (Game|SpawnActorfromClass "/Game/Enemy/Oriental/Raijin_GodOfThunder/Abilities/MeteorAttack/BP_MeteorAttack.BP_MeteorAttack_C" (Math|Transform|MakeTransform (Transformation|GetActorLocation (Variables|Default|GetPlayer))) "Undefined" 0 self "/Game/Enemy/Oriental/Raijin_GodOfThunder/Abilities/MeteorAttack/RJGE_MEADamage.RJGE_MEADamage_C" 0.0 "(TagName=\"Oriental.Enemy.Raijin.Ability.MeteorAttack.Damage\")" 0))

(event Custom|FlyAttackSpawnMeteor
  (bind _outactors (Actor|GetAllActorsOfClass "/Script/Escape_Game.GASCharacter"))
  (for _array_element _outactors
    (Utilities|IsValid _array_element
      (:Is%20Valid
        (Variables|Default|SetCurrentPlayer _array_element)
        (Game|SpawnActorfromClass "/Game/Enemy/Oriental/Raijin_GodOfThunder/Abilities/MeteorAttack/BP_MeteorAttack.BP_MeteorAttack_C" (Math|Transform|MakeTransform (Transformation|GetActorLocation (Variables|Default|GetCurrentPlayer))) "Undefined" 0 self "/Game/Enemy/Oriental/Raijin_GodOfThunder/Abilities/MeteorAttack/RJGE_MEADamage.RJGE_MEADamage_C" 0.0 "(TagName=\"Oriental.Enemy.Raijin.Ability.MeteorAttack.Damage\")" 0)
        (Development|PrintString "Spawning Meteor")))))

(event Custom|BurnPlayer
  (bind _outactors (Actor|GetAllActorsOfClass "/Script/Escape_Game.GASCharacter"))
  (for _array_element _outactors
    (Utilities|IsValid _array_element
      (:Is%20Valid
        (bind _output_get (Variables|Default|SetCurrentPlayer _array_element))
        (bind _returnvalue (Game|SpawnActorfromClass "/Game/Enemy/Oriental/Raijin_GodOfThunder/Abilities/FlyAttackBurn/BP_BurnAttack.BP_BurnAttack_C" (Transformation|GetSocketTransform (Variables|/Script/Engine.Character|GetMesh (Variables|Default|GetCurrentPlayer)) "ik_hand_root" "RTS_World") "Undefined" 0 self _output_get 0))
        (Transformation|AttachComponentToComponent _returnvalue (Variables|/Script/Engine.Character|GetMesh (Variables|Default|GetCurrentPlayer)) "ik_hand_root" "SnapToTarget" "SnapToTarget" "SnapToTarget" true)))))

(event EventBeginPlay
  (|CallParentFunction)
  (Utilities|FlowControl|Sequence
    (:then_0
      (bind _returnvalue (Game|SpawnActorfromClass "/Game/Enemy/Oriental/Raijin_GodOfThunder/BP_RaijinWeaponL.BP_RaijinWeaponL_C" (Transformation|GetSocketTransform (Variables|Character|GetMesh) "weapon_lSocket" "RTS_World") "Undefined" 0 self 0))
      (bind _output_get (Variables|Default|SetWeaponL _returnvalue))
      (Transformation|AttachComponentToComponent _output_get (Variables|Character|GetMesh) "weapon_lSocket" "SnapToTarget" "SnapToTarget" "SnapToTarget" true))
    (:then_1
      (bind _returnvalue_2 (Game|SpawnActorfromClass "/Game/Enemy/Oriental/Raijin_GodOfThunder/BP_RaijinWeaponR.BP_RaijinWeaponR_C" (Transformation|GetSocketTransform (Variables|Character|GetMesh) "weapon_rSocket" "RTS_World") "Undefined" 0 self 0))
      (bind _output_get_2 (Variables|Default|SetWeaponR _returnvalue_2))
      (Transformation|AttachComponentToComponent _output_get_2 (Variables|Character|GetMesh) "weapon_rSocket" "SnapToTarget" "SnapToTarget" "SnapToTarget" true))))

(event Collision|EventActorBeginOverlap
  (params (OtherActor :type Actor%20Object%20Reference)))

(event EventTick
  (params (DeltaSeconds :type Float%20%28single-precision%29))
  (Variables|Default|SetHealth (.ReturnValue (Ability|Attribute|GetFloatAttributefromAbilitySystemComponent (Variables|Default|GetAbilitySystemComponent) "(AttributeName=\"Health\",Attribute=/Script/Escape_Game.GASAttributeSet:Health,AttributeOwner=Class'\"/Script/Escape_Game.GASAttributeSet\"')")))
  (Variables|Default|SetMaxHealth (.ReturnValue (Ability|Attribute|GetFloatAttributefromAbilitySystemComponent (Variables|Default|GetAbilitySystemComponent) "(AttributeName=\"MaxHealth\",Attribute=/Script/Escape_Game.GASAttributeSet:MaxHealth,AttributeOwner=Class'\"/Script/Escape_Game.GASAttributeSet\"')")))
  (|CallParentFunction DeltaSeconds)
  (if (<= (* (/ (Variables|Default|GetHealth) (Variables|Default|GetMaxHealth)) 1e+02) 75.0)
    (Utilities|FlowControl|DoOnce false
      (:Completed
        (Variables|Default|SetFlyingIdle true)
        (Utilities|FlowControl|Delay 2.0)
        (Variables|Default|SetFlyingAttack1 true)
        (Utilities|FlowControl|Delay 1.74)
        (Variables|Default|SetFlyingAttack1 false)
        (Utilities|FlowControl|Delay 3.0)
        (Variables|Default|SetFlyingAttack2 true)
        (Utilities|FlowControl|Delay 2.33)
        (Variables|Default|SetFlyingAttack2 false)
        (Utilities|FlowControl|Delay 3.0)
        (Variables|Default|SetFlyingIdle false)
        (Utilities|FlowControl|Delay 2.0)))))

(event EventAttackPlayer
  (Utilities|FlowControl|Delay 2.0)
  (Utilities|FlowControl|DoOnce false :!label _label
    (:Completed
      (Utilities|FlowControl|Delay 1.87)
      (bind _returnvalue (Abilities|TryActivateAbilitybyClass (Variables|Default|GetAbilitySystemComponent) "/Game/Enemy/Oriental/Raijin_GodOfThunder/Abilities/SpawnMeteor/RJGA_SpawnMeteor.RJGA_SpawnMeteor_C" true))
      (Variables|Default|SetCanCast2nd _returnvalue)
      (Utilities|FlowControl|Delay 2.0)
      (Variables|Default|SetCanCast2nd false)
      (Utilities|FlowControl|Delay 5.0)
      (bind _returnvalue_2 (Abilities|TryActivateAbilitybyClass (Variables|Default|GetAbilitySystemComponent) "/Game/Enemy/Oriental/Raijin_GodOfThunder/Abilities/MeteorAttack/RJGA_MeteorAttack.RJGA_MeteorAttack_C" true))
      (Variables|Default|SetCanCast3rd _returnvalue_2)
      (Utilities|FlowControl|Delay 0.95)
      (Variables|Default|SetCanCast3rd false)
      (goto _label Reset))))

(fn ConstructionScript)