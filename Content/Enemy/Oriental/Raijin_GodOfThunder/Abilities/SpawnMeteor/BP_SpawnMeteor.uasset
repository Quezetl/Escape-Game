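; BP_SpawnMeteor is an actor for the Raijin enemy's SpawnMeteor ability that damages GAS characters touching its sphere.
; On overlap begin, if its Raijin reference is valid, Raijin's ability system builds an RJGE_SMDamage spec and applies it to the character.
; The damage amount is fixed here and passed as a tag-keyed SetByCaller magnitude.
; The end-overlap handler only casts, and no spawning or movement logic appears in the graphs.
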(event OnComponentBeginOverlap(Sphere)
  (params (OverlappedComponent :type Primitive%20Component%20Object%20Reference) (OtherActor :type Actor%20Object%20Reference) (OtherComp :type Primitive%20Component%20Object%20Reference) (OtherBodyIndex :type Integer) (bFromSweep :type Boolean) (SweepResult :type Hit%20Result%20Structure%20%28by%20ref%29))
  (bind _asgascharacter (Utilities|Casting|CastToGASCharacter OtherActor))
  (Variables|Default|SetCharacter _asgascharacter)
  (Utilities|IsValid (Variables|Default|GetRaijin)
    (:Is%20Valid
      (bind _returnvalue (Ability|GameplayEffect|AssignTagSetbyCallerMagnitude (GameplayEffects|MakeOutgoingSpec :self (Ability|GetAbilitySystemComponent (Variables|Default|GetRaijin)) :GameplayEffectClass "/Game/Enemy/Oriental/Raijin_GodOfThunder/Abilities/SpawnMeteor/RJGE_SMDamage.RJGE_SMDamage_C") "(TagName=\"Oriental.Enemy.Raijin.Ability.SpawnMeteor.Damage\")" -1e+01))
      (GameplayEffects|ApplyGameplayEffectSpecToTarget (Ability|GetAbilitySystemComponent (Variables|Default|GetRaijin)) _returnvalue (Ability|GetAbilitySystemComponent (Variables|Default|GetCharacter))))))

(event OnComponentEndOverlap(Sphere)
  (params (OverlappedComponent :type Primitive%20Component%20Object%20Reference) (OtherActor :type Actor%20Object%20Reference) (OtherComp :type Primitive%20Component%20Object%20Reference) (OtherBodyIndex :type Integer))
  (Utilities|Casting|CastToGASCharacter OtherActor))

(event EventBeginPlay)

(event Collision|EventActorBeginOverlap
  (params (OtherActor :type Actor%20Object%20Reference)))

(event EventTick
  (params (DeltaSeconds :type Float%20%28single-precision%29)))

(fn ConstructionScript)