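; BP_MeteorAttack is the impact actor for Raijin's meteor attack, dealing area damage once when it spawns.
; On BeginPlay it sphere-overlaps nearby pawns, ignoring Raijin, and keeps valid GASCharacters.
; For each, Raijin's damage functions combine a percentage of base damage with a target attribute passed as armor.
; The negated result goes into a GameplayEffect spec via SetByCaller, applied from Raijin's Ability System Component to the target.
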(event EventBeginPlay
  (bind _outactors (Collision|SphereOverlapActors (Transformation|GetActorLocation) 5e+02 (Utilities|Array|MakeArray "ObjectTypeQuery3") 0 (Utilities|Array|MakeArray (Variables|Default|GetRaijin))))
  (for _array_element _outactors
    (bind _asgascharacter (Utilities|Casting|CastToGASCharacter _array_element))
    (Utilities|IsValid _asgascharacter
      (:Is%20Valid
        (Variables|Default|SetCharacter _asgascharacter)
        (Utilities|IsValid (Variables|Default|GetRaijin)
          (:Is%20Valid
            (bind _damage (Default|AttributeBaseDamage (Variables|Default|GetRaijin) 8.0 "(AttributeName=\"MaxMana\",Attribute=/Script/Escape_Game.GASAttributeSet:MaxMana,AttributeOwner=Class'\"/Script/Escape_Game.GASAttributeSet\"')"))
            (bind _total_damage (Default|DamageDealt (Variables|Default|GetRaijin) _damage (.ReturnValue (Ability|Attribute|GetFloatAttribute (Variables|Default|GetCharacter) "(AttributeName=\"Armor\",Attribute=/Script/Escape_Game.GASAttributeSet:Armor,AttributeOwner=Class'\"/Script/Escape_Game.GASAttributeSet\"')"))))
            (bind _returnvalue (Ability|GameplayEffect|AssignTagSetbyCallerMagnitude (GameplayEffects|MakeOutgoingSpec :self (Ability|GetAbilitySystemComponent (Variables|Default|GetRaijin)) :GameplayEffectClass (Variables|Default|GetGE)) (Variables|Default|GetTag) (* _total_damage -1.0)))
            (GameplayEffects|ApplyGameplayEffectSpecToTarget (Ability|GetAbilitySystemComponent (Variables|Default|GetRaijin)) _returnvalue (Ability|GetAbilitySystemComponent (Variables|Default|GetCharacter)))))))))

(event Collision|EventActorBeginOverlap
  (params (OtherActor :type Actor%20Object%20Reference)))

(event EventTick
  (params (DeltaSeconds :type Float%20%28single-precision%29)))

(fn ConstructionScript)