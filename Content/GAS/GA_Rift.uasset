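; Gameplay ability that lets the player pick a location and spawns a BP_Rift actor there.
; On activation it runs a WaitTargetData task with user confirmation, using a trace target actor and the REC_Rift reticle.
; On valid data, a blocking hit spawns the rift with a scan radius and the owner's instigator, otherwise it prints an error.
; Either result ends the ability; cancelled targeting has no handler, and cost and cooldown are never committed.
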(event Ability|EventActivateAbility
  (bind _data (|WaitTargetData :ConfirmationType "UserConfirmed" :Class "/Script/Escape_Game.GASTargetActor" :TraceRange 2.5e+03 :ReticleClass "/Game/GAS/REC_Rift.REC_Rift_C")
    (:then
      (Development|PrintString "Targeting Active"))
    (:ValidData
      (if (.bBlockingHit (Collision|BreakHitResult (Ability|TargetData|GetHitResultfromTargetData _data)))
        (Game|SpawnActorfromClass :Class "/Game/GAS/BP_Rift.BP_Rift_C" :SpawnTransform (Math|Transform|MakeTransform (.Location (Collision|BreakHitResult (Ability|TargetData|GetHitResultfromTargetData _data)))) :CollisionHandlingOverride "AlwaysSpawn" :Scan%20Radius 5e+02 :Target self :Instigator (Variables|/Script/Engine.Actor|GetInstigator (Ability|GetOwningActorfromActorInfo)))
        (else
          (Development|PrintString "Invalid target")))
      (Ability|EndAbility))))

(event Ability|EventOnEndAbility
  (params (bWasCancelled :type Boolean)))