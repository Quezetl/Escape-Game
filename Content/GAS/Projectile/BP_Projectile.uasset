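; Homing projectile for the GAS character that damages enemies through the Gameplay Ability System.
; Every half second it searches "Homing"-tagged GASEnemy actors for one nearer than the stored ClosestDistance and homes its movement on that BP_ParRegEnem's Scene component.
; Capsule overlap with a GASEnemy applies PGGE_PTDamage from the instigator, with damage set by caller tag, then destroys the projectile after a short delay.
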(event OnComponentBeginOverlap(Capsule)
  (params (OverlappedComponent :type Primitive%20Component%20Object%20Reference) (OtherActor :type Actor%20Object%20Reference) (OtherComp :type Primitive%20Component%20Object%20Reference) (OtherBodyIndex :type Integer) (bFromSweep :type Boolean) (SweepResult :type Hit%20Result%20Structure%20%28by%20ref%29))
  (bind _asgasenemy (Utilities|Casting|CastToGASEnemy OtherActor))
  (bind _returnvalue (Ability|GameplayEffect|AssignTagSetbyCallerMagnitude (GameplayEffects|MakeOutgoingSpec :self (Ability|GetAbilitySystemComponent (Variables|Default|GetChar)) :GameplayEffectClass "/Game/GAS/Projectile/PGGE_PTDamage.PGGE_PTDamage_C") "(TagName=\"MainCharacter.Gideon.Ability.Projectile.Damage\")" -3e+01))
  (GameplayEffects|ApplyGameplayEffectSpecToTarget (Variables|/Script/Escape_Game.GASCharacter|GetAbilitySystemComponent (Variables|Default|GetChar)) _returnvalue (Ability|GetAbilitySystemComponent _asgasenemy))
  (Utilities|FlowControl|Delay 1.0)
  (Actor|DestroyActor))

(event Custom|Lock%20On%20Enemy
  (bind _projectilemovement (Variables|Default|GetProjectileMovement))
  (bind _homing_target (CallFunction|FindHomingTarget))
  (Utilities|IsValid _homing_target
    (:Is%20Valid
      (Variables|/Script/Engine.ProjectileMovementComponent|SetHomingTargetComponent _projectilemovement _homing_target)
      (Variables|/Script/Engine.ProjectileMovementComponent|SetbIsHomingProjectile _projectilemovement true))))

(event EventBeginPlay
  (bind _asgas_character (Utilities|Casting|CastToGAS_Character (Game|GetInstigator)))
  (Variables|Default|SetChar _asgas_character)
  (CallFunction|LockonEnemy :!label _label)
  (Utilities|FlowControl|Delay 0.5)
  (goto _label))

(fn ConstructionScript)

(fn FindHomingTarget
  (bind _outactors (Actor|GetAllActorsOfClasswithTag "/Script/Escape_Game.GASEnemy" "Homing"))
  (for _array_element _outactors
    (Utilities|IsValid _array_element
      (:Is%20Valid
        (if (< (Math|Vector|VectorLength (- (Transformation|GetActorLocation _array_element) (Transformation|GetActorLocation))) (Variables|Default|GetClosestDistance))
          (Variables|Default|SetClosestDistance (Math|Vector|VectorLength (- (Transformation|GetActorLocation _array_element) (Transformation|GetActorLocation))))
          (bind _output_get (Variables|Default|SetHoming%20Target _array_element))
          (if (Actor|ActorHasTag _output_get "Flying Enemy")
            (bind _asbp_par_reg_enem (Utilities|Casting|CastToBP_ParRegEnem _output_get))
            (bind _output_get_2 (Variables|Default|SetEnemy _asbp_par_reg_enem))
            (Variables|Default|SetSceneComp (Variables|/Game/GASEnemy/BP_ParRegEnem.BP_ParRegEnem_C|GetScene _output_get_2))
            (else
              (bind _asbp_par_reg_enem_2 (Utilities|Casting|CastToBP_ParRegEnem _output_get))
              (bind _output_get_3 (Variables|Default|SetEnemy _asbp_par_reg_enem_2))
              (Variables|Default|SetSceneComp (Variables|/Game/GASEnemy/BP_ParRegEnem.BP_ParRegEnem_C|GetScene _output_get_3))))))))
  (Utilities|IsValid (Variables|Default|GetSceneComp)
    (:Is%20Valid
      (return (Variables|Default|GetSceneComp)))))