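; BP_Rift is a GAS area-damage actor that strikes nearby pawns once, when it spawns.
; On BeginPlay it sphere-scans around itself, excluding its instigator, for pawns with an Ability System Component.
; DamageDealt weighs an instigator attribute against each pawn's armor using a two-branch formula, and prints the result.
; The negated damage goes into a GE_Rift spec as a SetByCaller magnitude, applied through the instigator's ability system.
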(event EventBeginPlay
  (bind _returnvalue (Game|GetInstigator))
  (bind _target (Variables|Default|GetTarget))
  (bind _outactors (Collision|SphereOverlapActors (Transformation|GetActorLocation) (Variables|Default|GetScan%20Radius) (Utilities|Array|MakeArray "ObjectTypeQuery3") 0 (Utilities|Array|MakeArray _returnvalue)))
  (for _array_element _outactors
    (Utilities|IsValid (Ability|GetAbilitySystemComponent _array_element)
      (:Is%20Valid
        (Utilities|IsValid _target
          (:Is%20Valid
            (bind _total_damage (CallFunction|DamageDealt (.ReturnValue (Ability|Attribute|GetFloatAttribute _returnvalue "(AttributeName=\"BaseAttackDamage\",Attribute=/Script/Escape_Game.GASAttributeSet:BaseAttackDamage,AttributeOwner=Class'\"/Script/Escape_Game.GASAttributeSet\"')")) (.ReturnValue (Ability|Attribute|GetFloatAttribute _array_element "(AttributeName=\"Armor\",Attribute=/Script/Escape_Game.GASAttributeSet:Armor,AttributeOwner=Class'\"/Script/Escape_Game.GASAttributeSet\"')"))))
            (bind _returnvalue_2 (Ability|GameplayEffect|AssignTagSetbyCallerMagnitude (Ability|MakeOutgoingGameplayEffectSpec _target "/Game/GAS/GE_Rift.GE_Rift_C") "(TagName=\"ability.rift\")" (* _total_damage -1.0)))
            (GameplayEffects|ApplyGameplayEffectSpecToTarget (Ability|GetAbilitySystemComponent _returnvalue) _returnvalue_2 (Ability|GetAbilitySystemComponent _array_element))))))))

(fn ConstructionScript)

(fn DamageDealt
  (params (Current%20Damage :type Float%20%28double-precision%29) (Enemy%20Armor :type Float%20%28double-precision%29))
  (bind _returnvalue (* Current%20Damage 2.0))
  (bind _returnvalue_2 (/ Current%20Damage Enemy%20Armor))
  (bind _returnvalue_3 (- _returnvalue Enemy%20Armor))
  (bind _returnvalue_4 (* _returnvalue_2 Current%20Damage))
  (if (>= Current%20Damage Enemy%20Armor)
    (Development|PrintString (Utilities|String|ToString(Text) (Utilities|Text|FormatText "Damage: {dmg}" _returnvalue_3)))
    (return _returnvalue_3)
    (else
      (Development|PrintString (Utilities|String|ToString(Text) (Utilities|Text|FormatText "Damage\" {dmg}" _returnvalue_4)))
      (return _returnvalue_4))))