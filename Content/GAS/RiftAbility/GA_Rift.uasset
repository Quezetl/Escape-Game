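; Gameplay ability that lets the player pick a spot with a targeting actor and reticle, then spawns a BP_Rift there.
; It waits for user-confirmed target data, commits, and spawns the rift with a scan radius on a blocking hit, otherwise printing an invalid-target message.
; After confirmation it ends and clears the GAS_Character's ActivatingAbility flag; cancelling only ends the ability.
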(event Ability|EventActivateAbility
  (bind _data (|WaitTargetData :ConfirmationType "UserConfirmed" :Class "/Script/Escape_Game.GASTargetActor" :TraceRange 2.5e+03 :ReticleClass "/Game/GAS/RiftAbility/REC_Rift.REC_Rift_C")
    (:ValidData
      (Ability|CommitAbility)
      (if (.bBlockingHit (Collision|BreakHitResult (Ability|TargetData|GetHitResultfromTargetData _data)))
        (Game|SpawnActorfromClass :Class "/Game/GAS/RiftAbility/BP_Rift.BP_Rift_C" :SpawnTransform (Math|Transform|MakeTransform (.Location (Collision|BreakHitResult (Ability|TargetData|GetHitResultfromTargetData _data)))) :CollisionHandlingOverride "AlwaysSpawn" :Scan%20Radius 5e+02 :Target self :Instigator (Variables|/Script/Engine.Actor|GetInstigator (Ability|GetOwningActorfromActorInfo)))
        (else
          (Development|PrintString "Invalid target")))
      (Ability|EndAbility)
      (bind _asgas_character (Utilities|Casting|CastToGAS_Character (Ability|GetOwningActorfromActorInfo)))
      (Variables|/Game/GAS/GAS_Character.GAS_Character_C|SetActivatingAbility _asgas_character false))
    (:Cancelled
      (Ability|EndAbility))))

(event Ability|EventOnEndAbility
  (params (bWasCancelled :type Boolean)))