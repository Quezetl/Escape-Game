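; BP_Rift is a GAS rift ability actor that, on BeginPlay, sphere-scans nearby pawns except its instigator and damages regular enemies and two dragon types.
; DamageDealt weighs the instigator's attribute against enemy armor, and GASDealDamage applies the negated result through a GE_DamageRift spec using a SetByCaller tag.
; Regular enemies are also alerted to the instigator, and non-bosses flinch if still alive.
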(event EventBeginPlay
  ;[1 1 1] Check for ovelapping actors
  (bind _outactors (Collision|SphereOverlapActors (Transformation|GetActorLocation) (Variables|Default|GetScan%20Radius) (Utilities|Array|MakeArray "ObjectTypeQuery3") 0 (Utilities|Array|MakeArray (Game|GetInstigator))))
  (for _array_element _outactors
    (bind _asbp_par_reg_enem (Utilities|Casting|CastToBP_ParRegEnem _array_element)
      (:then
        (Utilities|IsValid _asbp_par_reg_enem
          (:Is%20Valid
            (bind _output_get (Variables|Default|SetEnemies _asbp_par_reg_enem))
            (CallFunction|GASDealDamage _output_get)
            (bind _result (CallFunction|EnemyNotDead (Variables|Default|GetEnemies)))
            (if (Actor|ActorHasTag (Variables|Default|GetEnemies) "Boss")
              _
              (else
                (Variables|/Game/GASEnemy/BP_ParRegEnem.BP_ParRegEnem_C|SetIsFlinching (Variables|Default|GetEnemies) _result)))
            (bind _asgascharacter (Utilities|Casting|CastToGASCharacter (Game|GetInstigator)))
            (Default|DetectPlayer (Variables|Default|GetEnemies) _asgascharacter))))
      (:CastFailed
        (bind _asbp_dragon_terror (Utilities|Casting|CastToBP_DragonTerror _array_element)
          (:then
            (Utilities|IsValid _asbp_dragon_terror
              (:Is%20Valid
                (bind _output_get_2 (Variables|Default|SetAs%20ABP%20Dragon%20Terror _asbp_dragon_terror))
                (CallFunction|GASDealDamage _output_get_2)
                (Development|PrintString "Hello"))))
          (:CastFailed
            (bind _asbp_dragon (Utilities|Casting|CastToBP_Dragon _array_element))
            (bind _output_get_3 (Variables|Default|SetMDragong _asbp_dragon))
            (CallFunction|GASDealDamage _output_get_3)
            (Development|PrintString "Medieval dragon getting damage")))))))

(fn ConstructionScript)

(fn DamageDealt
  (params (Current%20Damage :type Float%20%28double-precision%29) (Enemy%20Armor :type Float%20%28double-precision%29))
  (bind _returnvalue (* Current%20Damage 2.0))
  (bind _returnvalue_2 (/ Current%20Damage Enemy%20Armor))
  (bind _returnvalue_3 (- _returnvalue Enemy%20Armor))
  (bind _returnvalue_4 (* _returnvalue_2 Current%20Damage))
  (if (>= Current%20Damage Enemy%20Armor)
    (Development|PrintString (Utilities|String|ToString(Text) (Utilities|Text|FormatText "Damage: {dmg}" _returnvalue_3)))
    (return _returnvalue_3)
    (else
      (Development|PrintString (Utilities|String|ToString(Text) (Utilities|Text|FormatText "Damage\" {dmg}" _returnvalue_4)))
      (return _returnvalue_4))))

(fn GASDealDamage
  (params (Enemy :type GAS%20Enemy%20Object%20Reference))
  (bind _target (Variables|Default|GetTarget))
  ;[1 0.2812 0.2812] Apply Damage to Enemy
  (bind _total_damage (CallFunction|DamageDealt (.ReturnValue (Ability|Attribute|GetFloatAttribute (Game|GetInstigator) "(AttributeName=\"BaseAttackDamage\",Attribute=/Script/Escape_Game.GASAttributeSet:BaseAttackDamage,AttributeOwner=Class'\"/Script/Escape_Game.GASAttributeSet\"')")) (.ReturnValue (Ability|Attribute|GetFloatAttribute Enemy "(AttributeName=\"Armor\",Attribute=/Script/Escape_Game.GASAttributeSet:Armor,AttributeOwner=Class'\"/Script/Escape_Game.GASAttributeSet\"')"))))
  (Utilities|IsValid _target
    (:Is%20Valid
      (bind _returnvalue (Ability|GameplayEffect|AssignTagSetbyCallerMagnitude (Ability|MakeOutgoingGameplayEffectSpec _target "/Game/GAS/RiftAbility/GE_DamageRift.GE_DamageRift_C") "(TagName=\"ability.rift\")" (* _total_damage -1.0)))
      (GameplayEffects|ApplyGameplayEffectSpecToTarget (Ability|GetAbilitySystemComponent (Game|GetInstigator)) _returnvalue (Ability|GetAbilitySystemComponent Enemy)))))

(fn EnemyNotDead
  (params (Enemy :type GAS%20Enemy%20Object%20Reference))
  (return (!= 0.0 (.ReturnValue (Ability|Attribute|GetFloatAttributefromAbilitySystemComponent (Ability|GetAbilitySystemComponent Enemy) "(AttributeName=\"Health\",Attribute=/Script/Escape_Game.GASAttributeSet:Health,AttributeOwner=Class'\"/Script/Escape_Game.GASAttributeSet\"')")))))