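; Demo showcase character for the scorpion monster, with a mouse-driven orbit camera and spring-arm zoom.
; BeginPlay creates the CharacterDemoUI widget and binds its events to looping animation previews, morph target sliders and material cycling on ScorpionMesh.
; Leg thickness and spike controls apply one value across groups of morph targets.
; Randomize sets random morph weights and refreshes the sliders, while reset returns sliders and morphs to defaults.
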(event Custom|ChangeMat_event
  (bind _scorpionmaterials (Variables|Default|GetScorpionMaterials))
  ;[1 1 1] Material Events
  (Rendering|Material|SetMaterial (Variables|Default|GetScorpion_Mesh) 0 (Utilities|Array|Get(acopy) _scorpionmaterials (Variables|Default|GetScorpion%20Array%20Value)))
  (bind _result (Math|Integer|IncrementInt (Variables|Default|GetScorpion%20Array%20Value))
    (:%20%20
      (Math|Integer|CompareInt _result (Utilities|Array|LastIndex _scorpionmaterials)
        (:>
          (Variables|Default|SetScorpion%20Array%20Value 0))))))

(event Custom|ChangeLegThinkness+_event
  (params (SliderValue :type Float%20%28double-precision%29) (ArrayIndex :type Integer))
  ;[1 1 1] Change Morph Targets
  (for _array_element (Variables|/Game/Monsters/SFB_Scorpion/Blueprints/BP_WDG_CharacterDemoUI.BP_WDG_CharacterDemoUI_C|GetLegThickness+ (Variables|Default|GetCharacterDemo_UI))
    (Components|SkeletalMesh|SetMorphTarget (Variables|Default|GetScorpion_Mesh) _array_element SliderValue true)))

(event Custom|Attack1Anim_event
  ;[1 1 1] Animation Events
  (Components|Animation|PlayAnimation (Variables|Default|GetScorpion_Mesh) "/Game/Monsters/SFB_Scorpion/Animations/Anim_Attack_1.Anim_Attack_1" true))

(event Custom|ChangeLegThickness-_event
  (params (Slider%20Value :type Float%20%28double-precision%29) (Array%20Index :type Integer))
  ;[1 1 1] Change Morph Targets
  (for _array_element (Variables|/Game/Monsters/SFB_Scorpion/Blueprints/BP_WDG_CharacterDemoUI.BP_WDG_CharacterDemoUI_C|GetLegThickness- (Variables|Default|GetCharacterDemo_UI))
    (Components|SkeletalMesh|SetMorphTarget (Variables|Default|GetScorpion_Mesh) _array_element Slider%20Value true)))

(event Custom|ChangeLegSpikes-_event
  (params (Slider%20Value :type Float%20%28double-precision%29) (Array%20Index :type Integer))
  ;[1 1 1] Change Morph Targets
  (for _array_element (Variables|/Game/Monsters/SFB_Scorpion/Blueprints/BP_WDG_CharacterDemoUI.BP_WDG_CharacterDemoUI_C|GetLegSpikes- (Variables|Default|GetCharacterDemo_UI))
    (Components|SkeletalMesh|SetMorphTarget (Variables|Default|GetScorpion_Mesh) _array_element Slider%20Value true)))

(event Custom|Attack2Anim_event
  ;[1 1 1] Animation Events
  (Components|Animation|PlayAnimation (Variables|Default|GetScorpion_Mesh) "/Game/Monsters/SFB_Scorpion/Animations/Anim_Attack_2.Anim_Attack_2" true))

(event Custom|Attack3Anim_event
  ;[1 1 1] Animation Events
  (Components|Animation|PlayAnimation (Variables|Default|GetScorpion_Mesh) "/Game/Monsters/SFB_Scorpion/Animations/Anim_Attack_3.Anim_Attack_3" true))

(event Custom|Cast1Anim_event
  ;[1 1 1] Animation Events
  (Components|Animation|PlayAnimation (Variables|Default|GetScorpion_Mesh) "/Game/Monsters/SFB_Scorpion/Animations/Anim_Attack_1B.Anim_Attack_1B" true))

(event Custom|Cast2Anim_event
  ;[1 1 1] Animation Events
  (Components|Animation|PlayAnimation (Variables|Default|GetScorpion_Mesh) "/Game/Monsters/SFB_Scorpion/Animations/Anim_Attack_Idle.Anim_Attack_Idle" true))

(event Custom|TauntAnim_event
  ;[1 1 1] Animation Events
  (Components|Animation|PlayAnimation (Variables|Default|GetScorpion_Mesh) "/Game/Monsters/SFB_Scorpion/Animations/Anim_Taunt.Anim_Taunt" true))

(event Custom|BlockAnim_event
  ;[1 1 1] Animation Events
  (Components|Animation|PlayAnimation (Variables|Default|GetScorpion_Mesh) "/Game/Monsters/SFB_Scorpion/Animations/Anim_Dodge.Anim_Dodge" true))

(event Custom|HitAnim_event
  ;[1 1 1] Animation Events
  (Components|Animation|PlayAnimation (Variables|Default|GetScorpion_Mesh) "/Game/Monsters/SFB_Scorpion/Animations/Anim_Got_Hit.Anim_Got_Hit" true))

(event Custom|ChangeLegSpikes+_event
  (params (SliderValue :type Float%20%28double-precision%29) (ArrayIndex :type Integer))
  ;[1 1 1] Change Morph Targets
  (for _array_element (Variables|/Game/Monsters/SFB_Scorpion/Blueprints/BP_WDG_CharacterDemoUI.BP_WDG_CharacterDemoUI_C|GetLegSpikes+ (Variables|Default|GetCharacterDemo_UI))
    (Components|SkeletalMesh|SetMorphTarget (Variables|Default|GetScorpion_Mesh) _array_element SliderValue true)))

(event Custom|DieAnim_event
  ;[1 1 1] Animation Events
  (Components|Animation|PlayAnimation (Variables|Default|GetScorpion_Mesh) "/Game/Monsters/SFB_Scorpion/Animations/Anim_Death.Anim_Death" true))

(event Custom|BreakIdleLoopAnim_event
  ;[1 1 1] Animation Events
  (Components|Animation|PlayAnimation (Variables|Default|GetScorpion_Mesh) "/Game/Monsters/SFB_Scorpion/Animations/Anim_Idle_Break.Anim_Idle_Break" true))

(event Custom|IdleAnim_event
  ;[1 1 1] Animation Events
  (Components|Animation|PlayAnimation (Variables|Default|GetScorpion_Mesh) "/Game/Monsters/SFB_Scorpion/Animations/Anim_Idle.Anim_Idle" true))

(event Custom|WalkBackAnim_event
  ;[1 1 1] Animation Events
  (Components|Animation|PlayAnimation (Variables|Default|GetScorpion_Mesh) "/Game/Monsters/SFB_Scorpion/Animations/ScorpionAnims_Walk_Backward_RootM.ScorpionAnims_Walk_Backward_RootM" true))

(event Custom|WalkForwardAnim_event
  ;[1 1 1] Animation Events
  (Components|Animation|PlayAnimation (Variables|Default|GetScorpion_Mesh) "/Game/Monsters/SFB_Scorpion/Animations/ScorpionAnims_Walk_RootM.ScorpionAnims_Walk_RootM" true))

(event Custom|ResetBlendValues_event
  (params (ResetValue :type Float%20%28double-precision%29))
  ;[1 1 1] Randomize & Clear
  (bind _sliders (Default|MakeSliderArray (Variables|Default|GetCharacterDemo_UI)))
  (for _array_element _sliders
    (Class|Slider|SetValue _array_element ResetValue)
    (for _array_element_2 (Variables|Default|GetAllMorphTargets)
      (Components|SkeletalMesh|SetMorphTarget (Variables|Default|GetScorpion_Mesh) _array_element_2 0.0 false))))

(event Custom|ChangeMorphTarget_event
  (params (SliderValue :type Float%20%28double-precision%29) (ArrayIndex :type Integer))
  ;[1 1 1] Change Morph Targets
  (Components|SkeletalMesh|SetMorphTarget (Variables|Default|GetScorpion_Mesh) (Utilities|Array|Get(acopy) (Variables|Default|GetAllMorphTargets) ArrayIndex) SliderValue false))

(event Custom|RandomizeBlendValues_event
  (params (Random%20Value :type Float%20%28double-precision%29))
  (bind _returnvalue (Math|Random|RandomFloatinRange -1.0 1.0))
  ;[1 1 1] Randomize & Clear
  (for _array_element (Variables|Default|GetAllMorphTargets)
    (Components|SkeletalMesh|SetMorphTarget (Variables|Default|GetScorpion_Mesh) _array_element _returnvalue false))
  (bind _output_get (Variables|Default|SetLeg%20Thickness%20+%20Value _returnvalue))
  (for _array_element_2 (Variables|/Game/Monsters/SFB_Scorpion/Blueprints/BP_WDG_CharacterDemoUI.BP_WDG_CharacterDemoUI_C|GetLegThickness+ (Variables|Default|GetCharacterDemo_UI))
    (Components|SkeletalMesh|SetMorphTarget (Variables|Default|GetScorpion_Mesh) _array_element_2 _output_get true))
  (bind _output_get_2 (Variables|Default|SetLeg%20Thickness%20-%20Value _returnvalue))
  (for _array_element_3 (Variables|/Game/Monsters/SFB_Scorpion/Blueprints/BP_WDG_CharacterDemoUI.BP_WDG_CharacterDemoUI_C|GetLegThickness- (Variables|Default|GetCharacterDemo_UI))
    (Components|SkeletalMesh|SetMorphTarget (Variables|Default|GetScorpion_Mesh) _array_element_3 _output_get_2 true))
  (bind _output_get_3 (Variables|Default|SetLeg%20Spikes%20+%20Value _returnvalue))
  (for _array_element_4 (Variables|/Game/Monsters/SFB_Scorpion/Blueprints/BP_WDG_CharacterDemoUI.BP_WDG_CharacterDemoUI_C|GetLegSpikes+ (Variables|Default|GetCharacterDemo_UI))
    (Components|SkeletalMesh|SetMorphTarget (Variables|Default|GetScorpion_Mesh) _array_element_4 _output_get_3 true))
  (bind _output_get_4 (Variables|Default|SetLeg%20Spikes%20-%20Value _returnvalue))
  (for _array_element_5 (Variables|/Game/Monsters/SFB_Scorpion/Blueprints/BP_WDG_CharacterDemoUI.BP_WDG_CharacterDemoUI_C|GetLegSpikes- (Variables|Default|GetCharacterDemo_UI))
    (Components|SkeletalMesh|SetMorphTarget (Variables|Default|GetScorpion_Mesh) _array_element_5 _output_get_4 true)
    (Default|UpdateSliders (Variables|Default|GetCharacterDemo_UI) (Variables|Default|GetScorpion_Mesh) (Variables|Default|GetAllMorphTargets))))

(event EventBeginPlay
  ;[1 1 1] Show Mouse & Create Widget
  (bind _returnvalue (UserInterface|CreateWidget "/Game/Monsters/SFB_Scorpion/Blueprints/BP_WDG_CharacterDemoUI.BP_WDG_CharacterDemoUI_C"))
  (bind _output_get (Variables|Default|SetCharacterDemo_UI _returnvalue))
  (UserInterface|Viewport|AddtoViewport _output_get 0)
  (Variables|/Script/Engine.PlayerController|SetbShowMouseCursor (Game|GetPlayerController 0) true)
  ;[1 1 1] Change Morph Targets
  (EventDispatchers|BindEventtoChangeMorphTarget _returnvalue (delegate Custom|ChangeMorphTarget_event))
  (EventDispatchers|BindEventtoChangeAllLegsThickness+MorphTargetsEvent _returnvalue (delegate Custom|ChangeLegThinkness+_event))
  (EventDispatchers|BindEventtoChangeAllLegsThickness-MorphTargetsEvent _returnvalue (delegate Custom|ChangeLegThickness-_event))
  (EventDispatchers|BindEventtoChangeAllLegsSpikes+MorphTargetsEvent _returnvalue (delegate Custom|ChangeLegSpikes+_event))
  (EventDispatchers|BindEventtoChangeAllLegsSpikes-MorphTargetsEvent _returnvalue (delegate Custom|ChangeLegSpikes-_event))
  ;[1 1 1] Animation Events
  (EventDispatchers|BindEventtoAttack1AnimEvent _returnvalue (delegate Custom|Attack1Anim_event))
  (EventDispatchers|BindEventtoAttack2AnimEvent _returnvalue (delegate Custom|Attack2Anim_event))
  (EventDispatchers|BindEventtoAttack3AnimEvent _returnvalue (delegate Custom|Attack3Anim_event))
  (EventDispatchers|BindEventtoAttack1BAnimEvent _returnvalue (delegate Custom|Cast1Anim_event))
  (EventDispatchers|BindEventtoAttackIdleAnimEvent _returnvalue (delegate Custom|Cast2Anim_event))
  (EventDispatchers|BindEventtoTauntAnimEvent _returnvalue (delegate Custom|TauntAnim_event))
  (EventDispatchers|BindEventtoDodgeAnimEvent _returnvalue (delegate Custom|BlockAnim_event))
  (EventDispatchers|BindEventtoHitAnimEvent _returnvalue (delegate Custom|HitAnim_event))
  (EventDispatchers|BindEventtoDieAnimEvent _returnvalue (delegate Custom|DieAnim_event))
  (EventDispatchers|BindEventtoIdleBreakAnimEvent _returnvalue (delegate Custom|BreakIdleLoopAnim_event))
  (EventDispatchers|BindEventtoIdleAnimEvent _returnvalue (delegate Custom|IdleAnim_event))
  (EventDispatchers|BindEventtoWalkBackAnimEvent _returnvalue (delegate Custom|WalkBackAnim_event))
  (EventDispatchers|BindEventtoWalkForwardAnimEvent _returnvalue (delegate Custom|WalkForwardAnim_event))
  ;[1 1 1] Randomize & Clear
  (EventDispatchers|BindEventtoRandomiseBlendValuesEvent _returnvalue (delegate Custom|RandomizeBlendValues_event))
  (EventDispatchers|BindEventtoResetBlendValuesEvent _returnvalue (delegate Custom|ResetBlendValues_event))
  ;[1 1 1] Material Events
  (EventDispatchers|BindEventtoChangeMatEvent _returnvalue (delegate Custom|ChangeMat_event)))

(event Input|MouseEvents|MouseX
  (params (AxisValue :type Float%20%28single-precision%29))
  (bind _returnvalue (Pawn|GetControlRotation :!class /Script/Engine.Pawn))
  ;[1 1 1] Camera Movement
  (Pawn|Input|AddControllerYawInput AxisValue)
  (Pawn|SetControlRotation (Game|GetPlayerController 0) (Math|Rotator|MakeRotator 0.0 (.pitch _returnvalue) (.yaw _returnvalue))))

(event Input|MouseEvents|MouseY
  (params (AxisValue :type Float%20%28single-precision%29))
  ;[1 1 1] Camera Movement
  (Pawn|Input|AddControllerPitchInput AxisValue))

(event Input|MouseEvents|MouseWheelUp
  (params (Key :type Key%20Structure))
  (bind _springarm (Variables|Default|GetSpringArm))
  ;[1 1 1] Mouse Zoom
  (:Released
    (Variables|/Script/Engine.SpringArmComponent|SetTargetArmLength _springarm (Math|Float|Clamp(Float) (- (Variables|/Script/Engine.SpringArmComponent|GetTargetArmLength _springarm) 2e+01) (Variables|Default|GetMin) (Variables|Default|GetMax)))))

(event Input|MouseEvents|MouseWheelDown
  (params (Key :type Key%20Structure))
  (bind _springarm (Variables|Default|GetSpringArm))
  ;[1 1 1] Mouse Zoom
  (:Pressed
    (Variables|/Script/Engine.SpringArmComponent|SetTargetArmLength _springarm (Math|Float|Clamp(Float) (- (Variables|/Script/Engine.SpringArmComponent|GetTargetArmLength _springarm) -2e+01) (Variables|Default|GetMin) (Variables|Default|GetMax)))))

(fn ConstructionScript)

(fn ReadMorphTargetValues
  (bind _morphtargetswithlegvaluereference (Variables|Default|GetMorphTargetsWithLegValueReference))
  (return (Utilities|Array|MakeArray (Class|SkeletalMeshComponent|GetMorphTarget (Variables|Default|GetScorpion_Mesh) (Utilities|Array|Get(acopy) _morphtargetswithlegvaluereference)) (Class|SkeletalMeshComponent|GetMorphTarget (Variables|Default|GetScorpion_Mesh) (Utilities|Array|Get(acopy) _morphtargetswithlegvaluereference 1)) (Class|SkeletalMeshComponent|GetMorphTarget (Variables|Default|GetScorpion_Mesh) (Utilities|Array|Get(acopy) _morphtargetswithlegvaluereference 2)) (Class|SkeletalMeshComponent|GetMorphTarget (Variables|Default|GetScorpion_Mesh) (Utilities|Array|Get(acopy) _morphtargetswithlegvaluereference 3)) (Class|SkeletalMeshComponent|GetMorphTarget (Variables|Default|GetScorpion_Mesh) (Utilities|Array|Get(acopy) _morphtargetswithlegvaluereference 4)) (Class|SkeletalMeshComponent|GetMorphTarget (Variables|Default|GetScorpion_Mesh) (Utilities|Array|Get(acopy) _morphtargetswithlegvaluereference 5)) (Class|SkeletalMeshComponent|GetMorphTarget (Variables|Default|GetScorpion_Mesh) (Utilities|Array|Get(acopy) _morphtargetswithlegvaluereference 6)) (Class|SkeletalMeshComponent|GetMorphTarget (Variables|Default|GetScorpion_Mesh) (Utilities|Array|Get(acopy) _morphtargetswithlegvaluereference 7)) (Class|SkeletalMeshComponent|GetMorphTarget (Variables|Default|GetScorpion_Mesh) (Utilities|Array|Get(acopy) _morphtargetswithlegvaluereference 8)) (Class|SkeletalMeshComponent|GetMorphTarget (Variables|Default|GetScorpion_Mesh) (Utilities|Array|Get(acopy) _morphtargetswithlegvaluereference 9)) (Class|SkeletalMeshComponent|GetMorphTarget (Variables|Default|GetScorpion_Mesh) (Utilities|Array|Get(acopy) _morphtargetswithlegvaluereference 10)) (Class|SkeletalMeshComponent|GetMorphTarget (Variables|Default|GetScorpion_Mesh) (Utilities|Array|Get(acopy) _morphtargetswithlegvaluereference 11)) (Class|SkeletalMeshComponent|GetMorphTarget (Variables|Default|GetScorpion_Mesh) (Utilities|Array|Get(acopy) _morphtargetswithlegvaluereference 12)) (Class|SkeletalMeshComponent|GetMorphTarget (Variables|Default|GetScorpion_Mesh) (Utilities|Array|Get(acopy) _morphtargetswithlegvaluereference 13)) (Class|SkeletalMeshComponent|GetMorphTarget (Variables|Default|GetScorpion_Mesh) (Utilities|Array|Get(acopy) _morphtargetswithlegvaluereference 14)) (Class|SkeletalMeshComponent|GetMorphTarget (Variables|Default|GetScorpion_Mesh) (Utilities|Array|Get(acopy) _morphtargetswithlegvaluereference 15)) (Class|SkeletalMeshComponent|GetMorphTarget (Variables|Default|GetScorpion_Mesh) (Utilities|Array|Get(acopy) _morphtargetswithlegvaluereference 16)) (Class|SkeletalMeshComponent|GetMorphTarget (Variables|Default|GetScorpion_Mesh) (Utilities|Array|Get(acopy) _morphtargetswithlegvaluereference 17)) (Class|SkeletalMeshComponent|GetMorphTarget (Variables|Default|GetScorpion_Mesh) (Utilities|Array|Get(acopy) _morphtargetswithlegvaluereference 18)) (Class|SkeletalMeshComponent|GetMorphTarget (Variables|Default|GetScorpion_Mesh) (Utilities|Array|Get(acopy) _morphtargetswithlegvaluereference 19)) (Class|SkeletalMeshComponent|GetMorphTarget (Variables|Default|GetScorpion_Mesh) (Utilities|Array|Get(acopy) _morphtargetswithlegvaluereference 20)) (Class|SkeletalMeshComponent|GetMorphTarget (Variables|Default|GetScorpion_Mesh) (Utilities|Array|Get(acopy) _morphtargetswithlegvaluereference 21)) (Class|SkeletalMeshComponent|GetMorphTarget (Variables|Default|GetScorpion_Mesh) (Utilities|Array|Get(acopy) _morphtargetswithlegvaluereference 22)) (Class|SkeletalMeshComponent|GetMorphTarget (Variables|Default|GetScorpion_Mesh) (Utilities|Array|Get(acopy) _morphtargetswithlegvaluereference 23)) (Class|SkeletalMeshComponent|GetMorphTarget (Variables|Default|GetScorpion_Mesh) (Utilities|Array|Get(acopy) _morphtargetswithlegvaluereference 24)) (Class|SkeletalMeshComponent|GetMorphTarget (Variables|Default|GetScorpion_Mesh) (Utilities|Array|Get(acopy) _morphtargetswithlegvaluereference 25)) (Class|SkeletalMeshComponent|GetMorphTarget (Variables|Default|GetScorpion_Mesh) (Utilities|Array|Get(acopy) _morphtargetswithlegvaluereference 26)) (Class|SkeletalMeshComponent|GetMorphTarget (Variables|Default|GetScorpion_Mesh) (Utilities|Array|Get(acopy) _morphtargetswithlegvaluereference 27)) (Class|SkeletalMeshComponent|GetMorphTarget (Variables|Default|GetScorpion_Mesh) (Utilities|Array|Get(acopy) _morphtargetswithlegvaluereference 28)))))