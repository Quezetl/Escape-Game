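; Demo character for showcasing the Treant monster's animations, materials and morph targets, with mouse-driven camera rotation and clamped spring-arm zoom.
; On BeginPlay it creates the WDG_CharacterDemoUI widget, shows the cursor and binds the widget's events to its handlers.
; These handlers cycle looping animations with wraparound, rotate paired torso and limb materials, and set, randomize or reset morph targets.
; It also updates the widget's animation name and morph sliders.
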(event Custom|ChangeMorphTarget_event
  (params (SliderValue :type Float%20%28double-precision%29) (MorphTargetName :type Name) (ArrayIndex :type Integer))
  ;[1 1 1] Set Morph Targets
  (Components|SkeletalMesh|SetMorphTarget (Variables|Default|GetSkeletalMesh) MorphTargetName SliderValue true))

(event Custom|ChangeAnimCycle-
  (params (Subtraction :type Integer))
  ;[1 1 1] Animations
  (bind _output_get (Variables|Default|SetTreant%20Anim%20Array%20Value (+ (Variables|Default|GetTreant%20Anim%20Array%20Value) Subtraction)))
  (CallFunction|ChangeAnimation _output_get))

(event Custom|ChangeMaterial
  (bind _skeletalmesh (Variables|Default|GetSkeletalMesh))
  (bind _treanttorsomats (Variables|Default|GetTreantTorsoMats))
  ;[1 1 1] Materials
  (Rendering|Material|SetMaterial _skeletalmesh 1 (Utilities|Array|Get(acopy) _treanttorsomats (Variables|Default|GetTreant%20Mat%20Array%20Value)))
  (Rendering|Material|SetMaterial _skeletalmesh 0 (Utilities|Array|Get(acopy) (Variables|Default|GetTreantLimbMats) (Variables|Default|GetTreant%20Mat%20Array%20Value)))
  (bind _result (Math|Integer|IncrementInt (Variables|Default|GetTreant%20Mat%20Array%20Value))
    (:%20%20
      (Math|Integer|CompareInt _result (Utilities|Array|LastIndex _treanttorsomats)
        (:>
          (Variables|Default|SetTreant%20Mat%20Array%20Value 0))))))

(event Custom|PlayIdle_event
  (params (IdleAnim :type Anim%20Sequence%20Object%20Reference))
  ;[1 1 1] Animations
  (Components|Animation|PlayAnimation (Variables|Default|GetSkeletalMesh) IdleAnim true)
  (Rendering|Components|TextRender|SetText (Variables|/Game/Monsters/SFB_Treant/Blueprints/WDG_CharacterDemoUI.WDG_CharacterDemoUI_C|GetAnimationName (Variables|Default|GetCharacter%20Demo%20UI%20Widget)) (Utilities|Text|ToText(Object) "/Game/Monsters/SFB_Treant/Animations/Anim_Treant_PeacefulIdle.Anim_Treant_PeacefulIdle")))

(event Custom|RandomizeMorphValues_event
  (bind _character_demo_ui_widget (Variables|Default|GetCharacter%20Demo%20UI%20Widget))
  (bind _skeletalmesh (Variables|Default|GetSkeletalMesh))
  (bind _morphtargets (Variables|/Game/Monsters/SFB_Treant/Blueprints/WDG_CharacterDemoUI.WDG_CharacterDemoUI_C|GetMorphTargets _character_demo_ui_widget))
  ;[1 1 1] Morph Random & Reset
  (for _array_element _morphtargets
    (Components|SkeletalMesh|SetMorphTarget _skeletalmesh _array_element (Math|Random|RandomFloatinRange -1.0 1.0) false)
    (Default|UpdateSliders (Variables|Default|GetCharacter%20Demo%20UI%20Widget) _skeletalmesh _morphtargets)))

(event Custom|ResetMorphValues_event
  (params (ResetValue :type Float%20%28double-precision%29))
  ;[1 1 1] Morph Random & Reset
  (bind _sliders (Default|MakeSliderArray (Variables|Default|GetCharacter%20Demo%20UI%20Widget)))
  (bind _output_get (Variables|Default|SetSliders _sliders))
  (for _array_element _output_get
    (Class|Slider|SetValue _array_element ResetValue)
    (for _array_element_2 (Variables|/Game/Monsters/SFB_Treant/Blueprints/WDG_CharacterDemoUI.WDG_CharacterDemoUI_C|GetMorphTargets (Variables|Default|GetCharacter%20Demo%20UI%20Widget))
      (Components|SkeletalMesh|SetMorphTarget (Variables|Default|GetSkeletalMesh) _array_element_2 ResetValue false))))

(event Custom|ChangeAnimCycle+
  (params (Addition :type Integer))
  ;[1 1 1] Animations
  (bind _output_get (Variables|Default|SetTreant%20Anim%20Array%20Value (+ (Variables|Default|GetTreant%20Anim%20Array%20Value) Addition)))
  (CallFunction|ChangeAnimation _output_get))

(event EventBeginPlay
  ;[1 1 1] Show Mouse & Create Widget
  (bind _returnvalue (UserInterface|CreateWidget "/Game/Monsters/SFB_Treant/Blueprints/WDG_CharacterDemoUI.WDG_CharacterDemoUI_C"))
  (bind _output_get (Variables|Default|SetCharacter%20Demo%20UI%20Widget _returnvalue))
  (UserInterface|Viewport|AddtoViewport _output_get 0)
  (Variables|/Script/Engine.PlayerController|SetbShowMouseCursor (Game|GetPlayerController 0) true)
  ;[1 1 1] Animations
  (EventDispatchers|BindEventtoAnimCycle+ _returnvalue (delegate Custom|ChangeAnimCycle+))
  (EventDispatchers|BindEventtoAnimCycle- _returnvalue (delegate Custom|ChangeAnimCycle-))
  (EventDispatchers|BindEventtoPlayIdle _returnvalue (delegate Custom|PlayIdle_event))
  ;[1 1 1] Materials
  (EventDispatchers|BindEventtoChangeMatEvent _returnvalue (delegate Custom|ChangeMaterial))
  ;[1 1 1] Morph Random & Reset
  (EventDispatchers|BindEventtoRandomiseMorphValuesEvent _returnvalue (delegate Custom|RandomizeMorphValues_event))
  (EventDispatchers|BindEventtoResetMorphValuesEvent _returnvalue (delegate Custom|ResetMorphValues_event))
  ;[1 1 1] Set Morph Targets
  (EventDispatchers|BindEventtoChangeMorphTarget _returnvalue (delegate Custom|ChangeMorphTarget_event)))

(event Input|MouseEvents|MouseX
  (params (AxisValue :type Float%20%28single-precision%29))
  (bind _returnvalue (Pawn|GetControlRotation :!class /Script/Engine.Pawn))
  ;[1 1 1] Camera Movement
  (Pawn|Input|AddControllerYawInput AxisValue)
  (Pawn|SetControlRotation (Game|GetPlayerController 0) (Math|Rotator|MakeRotator 0.0 (.pitch _returnvalue) (.yaw _returnvalue))))

(event Input|MouseEvents|MouseY
  (params (AxisValue :type Float%20%28single-precision%29))
  ;[1 1 1] Camera Movement
  (Pawn|Input|AddControllerPitchInput AxisValue))

(event Input|MouseEvents|MouseWheelUp
  (params (Key :type Key%20Structure))
  (bind _springarm (Variables|Default|GetSpringArm))
  ;[1 1 1] Mouse Zoom
  (:Released
    (Variables|/Script/Engine.SpringArmComponent|SetTargetArmLength _springarm (Math|Float|Clamp(Float) (- (Variables|/Script/Engine.SpringArmComponent|GetTargetArmLength _springarm) 2e+01) (Variables|Default|GetMin) (Variables|Default|GetMax)))))

(event Input|MouseEvents|MouseWheelDown
  (params (Key :type Key%20Structure))
  (bind _springarm (Variables|Default|GetSpringArm))
  ;[1 1 1] Mouse Zoom
  (:Pressed
    (Variables|/Script/Engine.SpringArmComponent|SetTargetArmLength _springarm (Math|Float|Clamp(Float) (- (Variables|/Script/Engine.SpringArmComponent|GetTargetArmLength _springarm) -2e+01) (Variables|Default|GetMin) (Variables|Default|GetMax)))))

(fn ConstructionScript)

(fn ChangeAnimation
  (params (Index%20Value :type Integer))
  (bind _animations (Variables|Default|GetAnimations))
  (bind _animations_2 (Variables|Default|GetAnimations))
  (bind _returnvalue (Utilities|Array|LastIndex _animations))
  (bind _output (Utilities|Array|Get(acopy) _animations_2 Index%20Value))
  (Math|Integer|CompareInt Index%20Value _returnvalue
    (:>
      (bind _output_get (Variables|Default|SetTreant%20Anim%20Array%20Value 0))
      (Components|Animation|PlayAnimation (Variables|Default|GetSkeletalMesh) (Utilities|Array|Get(acopy) (Variables|Default|GetAnimations) _output_get) true)
      (Rendering|Components|TextRender|SetText (Variables|/Game/Monsters/SFB_Treant/Blueprints/WDG_CharacterDemoUI.WDG_CharacterDemoUI_C|GetAnimationName (Variables|Default|GetCharacter%20Demo%20UI%20Widget)) (Utilities|Text|ToText(Object) (Utilities|Array|Get(acopy) (Variables|Default|GetAnimations) _output_get))))
    (:==
      (Components|Animation|PlayAnimation (Variables|Default|GetSkeletalMesh) _output true :!label _label)
      (Rendering|Components|TextRender|SetText (Variables|/Game/Monsters/SFB_Treant/Blueprints/WDG_CharacterDemoUI.WDG_CharacterDemoUI_C|GetAnimationName (Variables|Default|GetCharacter%20Demo%20UI%20Widget)) (Utilities|Text|ToText(Object) _output)))
    (:<
      (Math|Integer|CompareInt Index%20Value
        (:>
          (goto _label))
        (:<
          (bind _output_get_2 (Variables|Default|SetTreant%20Anim%20Array%20Value _returnvalue))
          (Components|Animation|PlayAnimation (Variables|Default|GetSkeletalMesh) (Utilities|Array|Get(acopy) (Variables|Default|GetAnimations) _output_get_2) true)
          (Rendering|Components|TextRender|SetText (Variables|/Game/Monsters/SFB_Treant/Blueprints/WDG_CharacterDemoUI.WDG_CharacterDemoUI_C|GetAnimationName (Variables|Default|GetCharacter%20Demo%20UI%20Widget)) (Utilities|Text|ToText(Object) (Utilities|Array|Get(acopy) (Variables|Default|GetAnimations) _output_get_2)))))))
  (return))