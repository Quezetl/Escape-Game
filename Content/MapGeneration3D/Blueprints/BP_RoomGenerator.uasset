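; Room builder actor for 3D map generation that assembles a floor, perimeter walls and door gaps from RoomParameters.
; SpawnRoom adds a BP_FloorGenerator child actor, clamps the room to a minimum size and uses the returned edge and corner cells to place wall meshes.
; Enabled doors skip the wall at DoorIndex, derived from the left edge's midpoint for all sides.
; Dynamic materials tint boss and shop floors, and shops add a door-oriented chest.
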(event Custom|SpawnRoom
  (bind _returnvalue (Transformation|GetActorTransform))
  (bind _room_parameters (Variables|Default|GetRoom%20Parameters))
  (bind _room_parameters_2 (Variables|Default|GetRoom%20Parameters))
  (bind _room_parameters_3 (Variables|Default|GetRoom%20Parameters))
  (bind _room_parameters_4 (Variables|Default|GetRoom%20Parameters))
  (bind (_length _width _roomtype) (Utilities|Struct|BreakFRoom _room_parameters_2))
  (bind _door (Utilities|Struct|BreakFRoom _room_parameters_3))
  (bind _door_2 (Utilities|Struct|BreakFRoom _room_parameters))
  (bind (_length_2 _width_2) (Utilities|Struct|BreakFRoom _room_parameters_4))
  (bind (_location _rotation _scale) (Math|Transform|BreakTransform _returnvalue))
  (bind (_door_l _door_r _door_b _door_f) (Utilities|Struct|BreakFDoor _door))
  ;[1 1 1] Spawn floor
  (bind _returnvalue_2 (AddComponent|AddChildActorComponent false _returnvalue))
  (bind (_corners_cells _cell_left _cell_right _cell_back _cell_forward _floor) (Default|SpawnFloor (.AsBP%20Floor%20Generator (Utilities|Casting|CastToBP_FloorGenerator (Variables|/Script/Engine.ChildActorComponent|GetChildActor _returnvalue_2))) (select (< _length 3) 3 _length) (select (< _width 3) 3 _width) _scale _location))
  (Variables|Default|SetDoor%20Index (/ (Utilities|Array|Length _cell_left) 2))
  ;[1 0 0 1 26] Generation of different types of rooms
  (switch Utilities|FlowControl|Switch|SwitchonERoomType _roomtype
    (:NewEnumerator0
      _)
    (:NewEnumerator1
      ;[1 1 1] Boss room floor
      (for _array_element _floor
        (bind _returnvalue_3 (Rendering|Material|CreateDynamicMaterialInstance (.AsStatic%20Mesh%20Component (Utilities|Casting|CastToStaticMeshComponent _array_element)) 0 (Rendering|Material|GetMaterial (.AsStatic%20Mesh%20Component (Utilities|Casting|CastToStaticMeshComponent _array_element)) 0) "None" :!class /Script/Engine.PrimitiveComponent))
        (Rendering|Material|SetVectorParameterValue _returnvalue_3 "TopSurfaceColor" "(R=0.623264,G=0.042200,B=0.044210,A=1.000000)" :!class /Script/Engine.MaterialInstanceDynamic)))
    (:NewEnumerator2
      ;[1 1 1] Item shop floor
      (for _array_element_2 _floor
        (bind _returnvalue_4 (Rendering|Material|CreateDynamicMaterialInstance (.AsStatic%20Mesh%20Component (Utilities|Casting|CastToStaticMeshComponent _array_element_2)) 0 (Rendering|Material|GetMaterial (.AsStatic%20Mesh%20Component (Utilities|Casting|CastToStaticMeshComponent _array_element_2)) 0) "None" :!class /Script/Engine.PrimitiveComponent))
        (Rendering|Material|SetVectorParameterValue _returnvalue_4 "TopSurfaceColor" "(R=1.000000,G=0.885968,B=0.073573,A=1.000000)" :!class /Script/Engine.MaterialInstanceDynamic))
      (AddComponent|AddStaticMeshComponent false (Math|Transform|MakeTransform (Math|Vector|MakeVector (+ (.X (Math|Vector|BreakVector (Transformation|GetActorLocation (.AsBP%20Floor%20Generator (Utilities|Casting|CastToBP_FloorGenerator (Variables|/Script/Engine.ChildActorComponent|GetChildActor _returnvalue_2)))))) (* (- (Math|Conversions|ToFloat(Integer) _length_2) 1.0) 1e+02)) (+ (.Y (Math|Vector|BreakVector (Transformation|GetActorLocation (.AsBP%20Floor%20Generator (Utilities|Casting|CastToBP_FloorGenerator (Variables|/Script/Engine.ChildActorComponent|GetChildActor _returnvalue_2)))))) (* (- (Math|Conversions|ToFloat(Integer) _width_2) 1.0) 1e+02)) (+ (.Z (Math|Vector|BreakVector (Transformation|GetActorLocation (.AsBP%20Floor%20Generator (Utilities|Casting|CastToBP_FloorGenerator (Variables|/Script/Engine.ChildActorComponent|GetChildActor _returnvalue_2)))))) 15.0)) (select (.door_l _door_2) "0.000000,-180.000000,0.000000" (select (.door_r _door_2) "0, 0, 0" (select (.door_b _door_2) "0,90.000000, 0" "0,-90.000000, 0"))) "2.000000,2.000000,2.000000"))))
  (for (_array_element_3 _array_index) _corners_cells
    ;[1 1 1] Wall Corners
    (if (== _array_index 0)
      (CallFunction|SpawnBackWall (Transformation|GetWorldLocation (Utilities|Array|Get(acopy) _floor _array_element_3)))
      (CallFunction|SpawnLeftWall (Transformation|GetWorldLocation (Utilities|Array|Get(acopy) _floor _array_element_3)))
      (elif (== _array_index 2)
        (CallFunction|SpawnBackWall (Transformation|GetWorldLocation (Utilities|Array|Get(acopy) _floor _array_element_3)))
        (CallFunction|SpawnRightWall (Transformation|GetWorldLocation (Utilities|Array|Get(acopy) _floor _array_element_3)))
        (elif (== _array_index 3)
          (CallFunction|SpawnForwardWall (Transformation|GetWorldLocation (Utilities|Array|Get(acopy) _floor _array_element_3)))
          (CallFunction|SpawnRightWall (Transformation|GetWorldLocation (Utilities|Array|Get(acopy) _floor _array_element_3)))
          (elif (== _array_index 1)
            (CallFunction|SpawnForwardWall (Transformation|GetWorldLocation (Utilities|Array|Get(acopy) _floor _array_element_3)))
            (CallFunction|SpawnLeftWall (Transformation|GetWorldLocation (Utilities|Array|Get(acopy) _floor _array_element_3))))))))
  ;[1 1 1] Set doors
  ;;[1 1 1] Left Door
  (for (_array_element_4 _array_index_2) _cell_left
    (if (not (and _door_l (== _array_index_2 (Variables|Default|GetDoor%20Index))))
      (CallFunction|SpawnLeftWall (Transformation|GetWorldLocation (Utilities|Array|Get(acopy) _floor _array_element_4)))))
  ;;[1 1 1] Right Door
  (for (_array_element_5 _array_index_3) _cell_right
    (if (not (and _door_r (== _array_index_3 (Variables|Default|GetDoor%20Index))))
      (CallFunction|SpawnRightWall (Transformation|GetWorldLocation (Utilities|Array|Get(acopy) _floor _array_element_5)))))
  ;;[1 1 1] Back Door
  (for (_array_element_6 _array_index_4) _cell_back
    (if (not (and _door_b (== _array_index_4 (Variables|Default|GetDoor%20Index))))
      (CallFunction|SpawnBackWall (Transformation|GetWorldLocation (Utilities|Array|Get(acopy) _floor _array_element_6)))))
  ;;[1 1 1] Forward Door
  (for (_array_element_7 _array_index_5) _cell_forward
    (if (not (and _door_f (== _array_index_5 (Variables|Default|GetDoor%20Index))))
      (CallFunction|SpawnForwardWall (Transformation|GetWorldLocation (Utilities|Array|Get(acopy) _floor _array_element_7))))))

(fn ConstructionScript)

(fn SpawnBackWall
  (params (FloorLocation :type Vector))
  (bind _returnvalue (Transformation|GetActorTransform))
  (bind (_location _rotation _scale) (Math|Transform|BreakTransform _returnvalue))
  (bind _returnvalue_2 (AddComponent|AddStaticMeshComponent false (Math|Transform|MakeTransform (- (- FloorLocation "48.000000,0.000000,20.000000") _location) _rotation _scale)))
  (Components|StaticMesh|SetStaticMesh _returnvalue_2 "/Game/MapGeneration3D/Meshes/DefaultWall.DefaultWall"))

(fn SpawnForwardWall
  (params (FloorLocation :type Vector))
  (bind _returnvalue (Transformation|GetActorTransform))
  (bind (_location _rotation _scale) (Math|Transform|BreakTransform _returnvalue))
  (bind (_roll _pitch _yaw) (Math|Rotator|BreakRotator _rotation))
  (bind _returnvalue_2 (AddComponent|AddStaticMeshComponent false (Math|Transform|MakeTransform (- (- FloorLocation "-96.000000,0.000000,20.000000") _location) (Math|Rotator|MakeRotator _roll _pitch (- _yaw 0.0)) _scale)))
  (Components|StaticMesh|SetStaticMesh _returnvalue_2 "/Game/MapGeneration3D/Meshes/DefaultWall.DefaultWall"))

(fn SpawnLeftWall
  (params (FloorLocation :type Vector))
  (bind _returnvalue (Transformation|GetActorTransform))
  (bind (_location _rotation _scale) (Math|Transform|BreakTransform _returnvalue))
  (bind (_roll _pitch _yaw) (Math|Rotator|BreakRotator _rotation))
  (bind _returnvalue_2 (AddComponent|AddStaticMeshComponent false (Math|Transform|MakeTransform (- (- FloorLocation "0.000000,96.000000,20.000000") _location) (Math|Rotator|MakeRotator _roll _pitch (- _yaw 9e+01)) _scale)))
  (Components|StaticMesh|SetStaticMesh _returnvalue_2 "/Game/MapGeneration3D/Meshes/DefaultWall.DefaultWall"))

(fn SpawnRightWall
  (params (FloorLocation :type Vector))
  (bind _returnvalue (Transformation|GetActorTransform))
  (bind (_location _rotation _scale) (Math|Transform|BreakTransform _returnvalue))
  (bind (_roll _pitch _yaw) (Math|Rotator|BreakRotator _rotation))
  (bind _returnvalue_2 (AddComponent|AddStaticMeshComponent false (Math|Transform|MakeTransform (- (- FloorLocation "0.000000,-48.000000,20.000000") _location) (Math|Rotator|MakeRotator _roll _pitch (- _yaw 9e+01)) _scale)))
  (Components|StaticMesh|SetStaticMesh _returnvalue_2 "/Game/MapGeneration3D/Meshes/DefaultWall.DefaultWall"))