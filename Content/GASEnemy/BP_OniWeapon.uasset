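; BP_OniWeapon is the Oni enemy's weapon, which deals Gameplay Ability System damage to characters its hit box overlaps.
; CanDamage and CannotDamage events open and close the attack window, and hits are ignored while the Oni is flinching.
; A valid hit applies GE_EnemyAttack from the Oni's ability system to the target, passing damage as a tag-based SetByCaller magnitude.
; A DoOnce with a delayed reset limits hit frequency across all targets.
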(event OnComponentBeginOverlap(Box)
  (params (OverlappedComponent :type Primitive%20Component%20Object%20Reference) (OtherActor :type Actor%20Object%20Reference) (OtherComp :type Primitive%20Component%20Object%20Reference) (OtherBodyIndex :type Integer) (bFromSweep :type Boolean) (SweepResult :type Hit%20Result%20Structure%20%28by%20ref%29))
  (bind _bp_oni (Variables|Default|GetBP_Oni))
  (bind _returnvalue (Ability|GetAbilitySystemComponent _bp_oni))
  (bind _asgascharacter (Utilities|Casting|CastToGASCharacter OtherActor))
  (Utilities|IsValid (Ability|GetAbilitySystemComponent _asgascharacter)
    (:Is%20Valid
      (if (Variables|Default|GetCan%20Attack)
        (if (not (Variables|/Game/Enemy/Oriental/Oni/oni_BP.oni_BP_C|GetisFlinching (Variables|Default|GetBP_Oni)))
          (Utilities|FlowControl|DoOnce false :!label _label
            (:Completed
              (bind _returnvalue_2 (Ability|GameplayEffect|AssignTagSetbyCallerMagnitude (GameplayEffects|MakeOutgoingSpec :self _returnvalue :GameplayEffectClass "/Game/GAS/GE_EnemyAttack.GE_EnemyAttack_C") "(TagName=\"Enemy.NormalAttack.damage\")" -1e+01))
              (GameplayEffects|ApplyGameplayEffectSpecToTarget _returnvalue _returnvalue_2 (Ability|GetAbilitySystemComponent _asgascharacter))
              (Utilities|FlowControl|Delay 1.0)
              (goto _label Reset))))))))

(event EventBeginPlay)

(event Collision|EventActorBeginOverlap
  (params (OtherActor :type Actor%20Object%20Reference)))

(event EventTick
  (params (DeltaSeconds :type Float%20%28single-precision%29)))

(event EventCanDamage
  (Variables|Default|SetCan%20Attack true))

(event EventCannotDamage
  (Variables|Default|SetCan%20Attack false))

(fn ConstructionScript)