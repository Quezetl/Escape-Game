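; ShopKeeper NPC Blueprint that offers an open-shop prompt near its trigger and hosts the shop UI.
; Overlapping ShopTrigger creates the prompt widget, shows it if the shop is not already open, and removes it on exit.
; OpenShop swaps the prompt for a shop widget holding a reference to this NPC, disables character input, centers the cursor and switches to UI-only input.
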(event OnComponentEndOverlap(ShopTrigger)
  (params (OverlappedComponent :type Primitive%20Component%20Object%20Reference) (OtherActor :type Actor%20Object%20Reference) (OtherComp :type Primitive%20Component%20Object%20Reference) (OtherBodyIndex :type Integer))
  ;[1 1 1] Removing Open Shop UI from viewport
  (Utilities|Casting|CastTo OtherActor)
  (Variables|Default|SetIs%20Outside%20of%20Shop true)
  (Widget|RemovefromParent (stale OnComponentBeginOverlap(ShopTrigger) _returnvalue)))

(event OnComponentBeginOverlap(ShopTrigger)
  (params (OverlappedComponent :type Primitive%20Component%20Object%20Reference) (OtherActor :type Actor%20Object%20Reference) (OtherComp :type Primitive%20Component%20Object%20Reference) (OtherBodyIndex :type Integer) (bFromSweep :type Boolean) (SweepResult :type Hit%20Result%20Structure%20%28by%20ref%29))
  ;[1 1 1] Add Open Shop UI on viewport
  (Utilities|Casting|CastTo OtherActor)
  (bind _returnvalue (UserInterface|CreateWidget "/Game/Procedural_Level_Testing/ItemDrops/Widgets/OpenSHopUI.OpenSHopUI_C"))
  (bind _output_get (Variables|Default|SetOpenUI _returnvalue))
  (Variables|Default|SetIs%20Outside%20of%20Shop false)
  (if (not (Variables|Default|GetIs%20Shop%20Opened))
    (UserInterface|Viewport|AddtoViewport _output_get 0)))

(event Custom|Open%20Shop
  (bind _returnvalue (Game|GetPlayerController 0))
  (bind _returnvalue_2 (Viewport|GetViewportSize))
  ;[1 1 1] Opening the shop and set the game mode to UI
  (Variables|Default|SetIs%20Shop%20Opened true)
  (Widget|RemovefromParent (stale OnComponentBeginOverlap(ShopTrigger) _returnvalue))
  (bind _returnvalue_3 (UserInterface|CreateWidget "/Game/Procedural_Level_Testing/ItemDrops/Widgets/UI_Shop.UI_Shop_C" 0 self))
  (bind _output_get (Variables|Default|SetShopWidget _returnvalue_3))
  (UserInterface|Viewport|AddtoViewport _output_get 0)
  (Class|PlayerController|SetMouseLocation (Game|GetPlayerController 0) (Math|Float|Truncate (/ (.x _returnvalue_2) 2.0)) (Math|Float|Truncate (/ (.y _returnvalue_2) 2.0)))
  (Input|DisableInput (Game|GetPlayerCharacter 0) _returnvalue)
  (Input|SetInputModeUIOnly _returnvalue 0 "DoNotLock")
  (Variables|/Script/Engine.PlayerController|SetbShowMouseCursor _returnvalue true))

(fn ConstructionScript)