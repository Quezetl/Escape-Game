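; BP_FloorGenerator builds a rectangular grid of floor tiles for 3D procedural map generation.
; SpawnFloor adds static mesh components at fixed spacing, picking random meshes from FloorVariety with random quarter-turn yaw, unevenly weighted by nested coin flips.
; A running cell index sorts perimeter tiles into corner and Left, Right, Back, Forward edge arrays.
; It returns those arrays with the root's child components; the construction script is empty.
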(fn ConstructionScript)

(fn SpawnFloor
  (params (Lengh :type Integer) (Width :type Integer) (Scale :type Vector) (Location :type Vector))
  (bind _returnvalue (* Width Lengh))
  (bind _returnvalue_2 (* Lengh Width))
  (bind _floor_variety (Variables|Default|GetFloor%20Variety))
  (bind _i (LocalVariables|GetI))
  (bind _i_2 (LocalVariables|GetI))
  (bind _i_3 (LocalVariables|GetI))
  (bind _i_4 (LocalVariables|GetI))
  (bind _returnvalue_3 (< _i Width))
  (bind _returnvalue_4 (- _returnvalue Width))
  (bind _returnvalue_5 (- _returnvalue 1))
  (bind _returnvalue_6 (< _i _returnvalue_5))
  (bind _returnvalue_7 (> _i _returnvalue_4))
  (bind _returnvalue_8 (and _returnvalue_6 _returnvalue_7))
  (for _index (range 0 (- Lengh 1))
    (for _index_2 (range 0 (- Width 1))
      (bind _returnvalue_9 (AddComponent|AddStaticMeshComponent false (Math|Transform|MakeTransform (+ (Math|Vector|MakeVector (* _index_2 2e+02) (* _index 2e+02) 0.0) Location) (Math|Rotator|MakeRotator 0.0 0.0 (select (Math|Random|RandomBool) 9e+01 (select (Math|Random|RandomBool) 1.8e+02 (select (Math|Random|RandomBool) 2.7e+02 0.0)))) Scale)))
      (Components|StaticMesh|SetStaticMesh _returnvalue_9 (Utilities|Array|Get(acopy) _floor_variety (Math|Random|RandomIntegerinRange 0 (Utilities|Array|LastIndex _floor_variety))))
      ;[1 1 1] Corner cell search
      (if (Math|Boolean|ORBoolean _returnvalue_3 _returnvalue_8 (== _i (* Width _index)) (== _i (+ (* Width _index) (- Width 1))))
        (if (not (Math|Boolean|ORBoolean (== 0 _i_4) (== (- Width 1) _i_4) (== (- _returnvalue_2 1) _i_4) (== (- _returnvalue_2 Width) _i_4)))
          (if _returnvalue_3
            (Utilities|Array|Add (Variables|Default|GetCell_Left) _i_2)
            (elif _returnvalue_8
              (Utilities|Array|Add (Variables|Default|GetCell_Right) _i_2)
              (elif (== _i (* Width _index))
                (Utilities|Array|Add (Variables|Default|GetCell_Back) _i_3)
                (elif (== _i (+ (* Width _index) (- Width 1)))
                  (Utilities|Array|Add (Variables|Default|GetCell_Forward) _i_3)))))
          (else
            (Utilities|Array|Add (Variables|Default|GetCorners%20Cells) (LocalVariables|GetI)))))
      (Math|Integer|IncrementInt (LocalVariables|GetI))))
  (return (Variables|Default|GetCorners%20Cells) (Variables|Default|GetCell_Left) (Variables|Default|GetCell_Right) (Variables|Default|GetCell_Back) (Variables|Default|GetCell_Forward) (Components|GetChildrenComponents (Variables|Default|GetDefaultSceneRoot) false)))